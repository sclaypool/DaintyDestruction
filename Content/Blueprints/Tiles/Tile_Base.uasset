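; Base tile actor for a 2D side-scroller that flips from a bad sprite to a good one when the player touches it.
; The construction script sets the bad sprite.
; A box overlap with the 2DSideScrollerCharacter swaps to the good sprite and sets a Transformed flag, so the change happens only once.
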(event `self.ReceiveBeginPlay`)

(event `self.ReceiveActorBeginOverlap`
  (params (OtherActor :type "Actor Object Reference")))

(event `self.ReceiveTick`
  (params (DeltaSeconds :type "Float (single-precision)")))

(event `self.Box.OnComponentBeginOverlap`
  (params (OtherActor :type "Actor Object Reference") (OtherComp :type "PrimitiveComponent Object Reference") (OtherBodyIndex :type Integer) (bFromSweep :type Boolean) (SweepResult :type "HitResult Structure (by ref)"))
  (if (not (`self.Transformed`))
    (cast `/Game/Blueprints/2DSideScrollerCharacter` OtherActor)
    (`PaperSpriteComponent.SetSprite` (`self.PaperSprite`) (`self.GoodSprite`))
    (set `self.Transformed` true)))

(fn `UserConstructionScript`
  (`PaperSpriteComponent.SetSprite` (`self.PaperSprite`) (`self.BadSprite`)))