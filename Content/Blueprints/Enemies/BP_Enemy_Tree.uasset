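; Evil tree enemy for the 2D side-scroller that swipes at the player and can be transformed into a good tree.
; BeginPlay spawns two fist actors on the flipbook's damage sockets.
; Left and right triggers play swipe flipbooks, with Attacking set true halfway through via delays.
; Damage calls the parent, then plays a directional hit flipbook or, once Transformed, a flower explosion before idling as good and destroying the fists.
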(event `self.ReceiveBeginPlay`
  (bind _returnvalue (`KismetMathLibrary.MakeTransform` (0.0 0.0 0.0)))
  (bind _paperflipbook (`self.PaperFlipbook`))
  ;[1 1 1] Create fists to do damage
  (bind _returnvalue_2 (`|SpawnActorFromClass` "/Game/Blueprints/Enemies/BP_Tree_Fist.BP_Tree_Fist_C" _returnvalue "Undefined" "OverrideRootScale"))
  (`SceneComponent.K2_AttachTo` (`/Game/Blueprints/Enemies/BP_Tree_Fist.Sphere` _returnvalue_2) _paperflipbook "LeftDamage" "KeepRelativeOffset" true)
  (bind _returnvalue_3 (`|SpawnActorFromClass` "/Game/Blueprints/Enemies/BP_Tree_Fist.BP_Tree_Fist_C" _returnvalue "Undefined" "OverrideRootScale"))
  (`SceneComponent.K2_AttachTo` (`/Game/Blueprints/Enemies/BP_Tree_Fist.Sphere` _returnvalue_3) _paperflipbook "RightDamage" "KeepRelativeOffset" true))

(event `self.ReceiveActorBeginOverlap`
  (params (OtherActor :type "Actor Object Reference")))

(event `self.ReceiveTick`
  (params (DeltaSeconds :type "Float (single-precision)"))
  (`parent.ReceiveTick` 0.0))

(event `self.Damage`
  (params (AttackType :type "/Game/Blueprints/AttackType Enum" :default "NewEnumerator0"))
  ;[1 1 1] Process Tree Damage
  (`parent.Damage` AttackType)
  (if (`self.Transformed`)
    (`PrimitiveComponent.SetCollisionResponseToChannel` (`self.CapsuleComponent`) "ECC_Pawn" "ECR_Overlap")
    (`PaperFlipbookComponent.SetFlipbook` (`self.PaperFlipbook`) "/Game/Sprites/Flipbooks/FB_FlowerExplosion.FB_FlowerExplosion")
    (`self.PlayTransformSound`)
    (`SceneComponent.SetRelativeScale3D` (`self.PaperFlipbook`) (1.0 1.0 1.0))
    (`KismetSystemLibrary.Delay` (`PaperFlipbookComponent.GetFlipbookLength` (`self.PaperFlipbook`)))
    (`PaperFlipbookComponent.SetFlipbook` (`self.PaperFlipbook`) "/Game/Sprites/Flipbooks/TreeGood_Idle_Anim.TreeGood_Idle_Anim")
    (`self.K2_DestroyActor` (stale `self.ReceiveBeginPlay` _returnvalue_2))
    (`self.K2_DestroyActor` (stale `self.ReceiveBeginPlay` _returnvalue_3))
    (elif (`self.LeftAttack`)
      (`PaperFlipbookComponent.SetFlipbook` (`self.PaperFlipbook`) "/Game/Sprites/Flipbooks/FB_Tree_Evil_Hit_Left.FB_Tree_Evil_Hit_Left")
      (`KismetSystemLibrary.Delay` (`PaperFlipbookComponent.GetFlipbookLength` (`self.PaperFlipbook`)))
      (if (`self.Transformed`)
        (`PaperFlipbookComponent.SetFlipbook` (`self.PaperFlipbook`) "/Game/Sprites/Flipbooks/TreeGood_Idle_Anim.TreeGood_Idle_Anim")
        (else
          (`PaperFlipbookComponent.SetFlipbook` (`self.PaperFlipbook`) "/Game/Sprites/Flipbooks/FB_Tree_Evil_Idle.FB_Tree_Evil_Idle")))
      (else
        (`PaperFlipbookComponent.SetFlipbook` (`self.PaperFlipbook`) "/Game/Sprites/Flipbooks/FB_Tree_Evil_Hit_Right.FB_Tree_Evil_Hit_Right")
        (`KismetSystemLibrary.Delay` (`PaperFlipbookComponent.GetFlipbookLength` (`self.PaperFlipbook`)))
        (if (`self.Transformed`)
          (`PaperFlipbookComponent.SetFlipbook` (`self.PaperFlipbook`) "/Game/Sprites/Flipbooks/TreeGood_Idle_Anim.TreeGood_Idle_Anim")
          (else
            (`PaperFlipbookComponent.SetFlipbook` (`self.PaperFlipbook`) "/Game/Sprites/Flipbooks/FB_Tree_Evil_Idle.FB_Tree_Evil_Idle")))))))

(event `self.RightTrigger.OnComponentBeginOverlap`
  (params (OtherActor :type "Actor Object Reference") (OtherComp :type "PrimitiveComponent Object Reference") (OtherBodyIndex :type Integer) (bFromSweep :type Boolean) (SweepResult :type "HitResult Structure (by ref)"))
  (bind _returnvalue (/ (`PaperFlipbookComponent.GetFlipbookLength` (`self.PaperFlipbook`)) 2.0))
  ;[1 1 1] Right Attack
  (cast `/Game/Blueprints/2DSideScrollerCharacter` OtherActor)
  (if (and (not (`self.Attacking`)) (not (`self.RightTriggered`)) (not (`self.Transformed`)))
    (set `self.RightTriggered` true)
    (`self.ChangeAnimation` "/Game/Sprites/Flipbooks/FB_Tree_Evil_Swipe_Right.FB_Tree_Evil_Swipe_Right")
    (`KismetSystemLibrary.Delay` _returnvalue)
    (set `self.Attacking` true)
    (`KismetSystemLibrary.Delay` _returnvalue)
    (set `self.Attacking` false)))

(event `ChangeAnimation`
  (params (Flipbook :type "PaperFlipbook Object Reference"))
  (bind _paperflipbook (`self.PaperFlipbook`))
  ;[1 1 1] Change Animation
  (`PaperFlipbookComponent.SetFlipbook` _paperflipbook Flipbook)
  (`KismetSystemLibrary.Delay` (`PaperFlipbookComponent.GetFlipbookLength` _paperflipbook))
  (`PaperFlipbookComponent.SetFlipbook` _paperflipbook "/Game/Sprites/Flipbooks/FB_Tree_Evil_Idle.FB_Tree_Evil_Idle"))

(event `self.RightTrigger.OnComponentEndOverlap`
  (params (OtherActor :type "Actor Object Reference") (OtherComp :type "PrimitiveComponent Object Reference") (OtherBodyIndex :type Integer))
  ;[1 1 1] Right Attack
  (cast `/Game/Blueprints/2DSideScrollerCharacter` OtherActor)
  (set `self.RightTriggered` false))

(event `self.LeftTrigger.OnComponentBeginOverlap`
  (params (OtherActor :type "Actor Object Reference") (OtherComp :type "PrimitiveComponent Object Reference") (OtherBodyIndex :type Integer) (bFromSweep :type Boolean) (SweepResult :type "HitResult Structure (by ref)"))
  (bind _returnvalue (/ (`PaperFlipbookComponent.GetFlipbookLength` (`self.PaperFlipbook`)) 2.0))
  ;[1 1 1] Left Attack
  (cast `/Game/Blueprints/2DSideScrollerCharacter` OtherActor)
  (if (and (not (`self.Attacking`)) (not (`self.LeftTriggered`)) (not (`self.Transformed`)))
    (set `self.LeftTriggered` true)
    (`self.ChangeAnimation` "/Game/Sprites/Flipbooks/FB_Tree_Evil_Swipe_Left.FB_Tree_Evil_Swipe_Left")
    (`KismetSystemLibrary.Delay` _returnvalue)
    (set `self.Attacking` true)
    (`KismetSystemLibrary.Delay` _returnvalue)
    (set `self.Attacking` false)))

(event `self.LeftTrigger.OnComponentEndOverlap`
  (params (OtherActor :type "Actor Object Reference") (OtherComp :type "PrimitiveComponent Object Reference") (OtherBodyIndex :type Integer))
  ;[1 1 1] Left Attack
  (cast `/Game/Blueprints/2DSideScrollerCharacter` OtherActor)
  (if (not (`self.Attacking`))
    (set `self.LeftTriggered` false)))

(fn `UserConstructionScript`
  (`parent.UserConstructionScript`))