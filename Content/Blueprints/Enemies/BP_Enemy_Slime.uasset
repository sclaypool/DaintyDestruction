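; Paper2D slime enemy for a side-scroller that hops while idle and moves along X toward the player when detected.
; Tick launches each hop; OnLanded pauses on a delay, reversing direction if no player is detected.
; Left and right trigger overlaps set facing and enable movement input.
; Damage plays a hit flipbook or, once Transformed, overlaps Pawns and turns into a smaller walker after a flower explosion.
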(event `self.ReceiveBeginPlay`)

(event `self.ReceiveActorBeginOverlap`
  (params (OtherActor :type "Actor Object Reference")))

(event `self.ReceiveTick`
  (params (DeltaSeconds :type "Float (single-precision)"))
  (`parent.ReceiveTick` 0.0)
  (if (or (`self.LeftTriggered`) (`self.RightTriggered`))
    (`self.AddMovementInput` (1.0 0.0 0.0) (* (`self.Rotation`) (`self.MySpeed`)) true)
    (elif (and (`self.Idle`) (not (`self.Jiggle`)) (not (`self.Transformed`)))
      (set `self.Idle` false)
      (set `self.Jiggle` true)
      (`PaperFlipbookComponent.SetFlipbook` (`self.PaperFlipbook`) "/Game/Sprites/Flipbooks/ES_jiggle2.ES_jiggle2")
      (`self.LaunchCharacter` (`KismetMathLibrary.MakeVector` (* (`self.Rotation`) -200.0) 0.0 200.0))
      (elif (`self.Transformed`)
        _))))

(event `self.Damage`
  (params (AttackType :type "/Game/Blueprints/AttackType Enum" :default "NewEnumerator0"))
  ;[1 1 1] Transform
  (`parent.Damage` AttackType)
  (if (`self.Transformed`)
    (`PrimitiveComponent.SetCollisionResponseToChannel` (`self.CapsuleComponent`) "ECC_Pawn" "ECR_Overlap")
    (`PaperFlipbookComponent.SetFlipbook` (`self.PaperFlipbook`) "/Game/Sprites/Flipbooks/FB_FlowerExplosion.FB_FlowerExplosion")
    (`self.PlayTransformSound`)
    (`KismetSystemLibrary.Delay` (`PaperFlipbookComponent.GetFlipbookLength` (`self.PaperFlipbook`)))
    (`SceneComponent.SetRelativeScale3D` (`self.PaperFlipbook`) (0.6 0.6 0.6))
    (`PaperFlipbookComponent.SetFlipbook` (`self.PaperFlipbook`) "/Game/Sprites/Flipbooks/GT_walk2.GT_walk2")
    (else
      (`PaperFlipbookComponent.SetFlipbook` (`self.PaperFlipbook`) "/Game/Sprites/Flipbooks/ES_hit2.ES_hit2")
      (`KismetSystemLibrary.Delay` (`PaperFlipbookComponent.GetFlipbookLength` (`self.PaperFlipbook`)))
      (if (`self.Transformed`)
        (`PaperFlipbookComponent.SetFlipbook` (`self.PaperFlipbook`) "/Game/Sprites/Flipbooks/GT_walk2.GT_walk2")
        (else
          (`PaperFlipbookComponent.SetFlipbook` (`self.PaperFlipbook`) "/Game/Sprites/Flipbooks/ES_jiggle2.ES_jiggle2"))))))

(event `self.OnLanded`
  (params (Hit :type "HitResult Structure (by ref)"))
  ;[1 1 1] Slime Jiggle/Jump
  (set `self.Jiggle` false)
  (`PaperFlipbookComponent.SetFlipbook` (`self.PaperFlipbook`) "/Game/Sprites/Flipbooks/ES_Idle.ES_Idle")
  (if (> (`self.Rotation`) 0.0)
    (`SceneComponent.K2_SetRelativeRotation` (`self.PaperFlipbook`) (struct) false false)
    (else
      (`SceneComponent.K2_SetRelativeRotation` (`self.PaperFlipbook`) (struct :`Yaw` 180.0) false false)))
  (`KismetSystemLibrary.Delay` (* (`PaperFlipbookComponent.GetFlipbookLength` (`self.PaperFlipbook`)) 2.0))
  (if (and (not (`self.LeftTriggered`)) (not (`self.RightTriggered`)))
    (set `self.Rotation` (* (`self.Rotation`) -1.0)))
  (set `self.Idle` true))

(event `self.Left Trigger.OnComponentBeginOverlap`
  (params (OtherActor :type "Actor Object Reference") (OtherComp :type "PrimitiveComponent Object Reference") (OtherBodyIndex :type Integer) (bFromSweep :type Boolean) (SweepResult :type "HitResult Structure (by ref)"))
  ;[1 1 1] Left Overlap
  (cast `/Game/Blueprints/2DSideScrollerCharacter` OtherActor)
  (set `self.LeftTriggered` true)
  (`SceneComponent.K2_SetRelativeRotation` (`self.PaperFlipbook`) (struct :`Yaw` 180.0) false false)
  (set `self.Rotation` -1.0)
  (if (`self.Transformed`)
    (`PaperFlipbookComponent.SetFlipbook` (`self.PaperFlipbook`) "/Game/Sprites/Flipbooks/GT_walk2.GT_walk2")))

(event `self.Left Trigger.OnComponentEndOverlap`
  (params (OtherActor :type "Actor Object Reference") (OtherComp :type "PrimitiveComponent Object Reference") (OtherBodyIndex :type Integer))
  ;[1 1 1] Left Overlap
  (cast `/Game/Blueprints/2DSideScrollerCharacter` OtherActor)
  (set `self.LeftTriggered` false)
  (if (`self.Transformed`)
    (`PaperFlipbookComponent.SetFlipbook` (`self.PaperFlipbook`) "/Game/Sprites/Flipbooks/GT_idle2.GT_idle2")))

(event `self.Right Trigger.OnComponentBeginOverlap`
  (params (OtherActor :type "Actor Object Reference") (OtherComp :type "PrimitiveComponent Object Reference") (OtherBodyIndex :type Integer) (bFromSweep :type Boolean) (SweepResult :type "HitResult Structure (by ref)"))
  ;[1 1 1] Right Overlap
  (cast `/Game/Blueprints/2DSideScrollerCharacter` OtherActor)
  (set `self.RightTriggered` true)
  (`SceneComponent.K2_SetRelativeRotation` :`self` (`self.PaperFlipbook`))
  (set `self.Rotation` 1.0)
  (if (`self.Transformed`)
    (`PaperFlipbookComponent.SetFlipbook` (`self.PaperFlipbook`) "/Game/Sprites/Flipbooks/GT_walk2.GT_walk2")))

(event `self.Right Trigger.OnComponentEndOverlap`
  (params (OtherActor :type "Actor Object Reference") (OtherComp :type "PrimitiveComponent Object Reference") (OtherBodyIndex :type Integer))
  ;[1 1 1] Right Overlap
  (cast `/Game/Blueprints/2DSideScrollerCharacter` OtherActor)
  (set `self.RightTriggered` false)
  (if (`self.Transformed`)
    (`PaperFlipbookComponent.SetFlipbook` (`self.PaperFlipbook`) "/Game/Sprites/Flipbooks/GT_idle2.GT_idle2")))

(fn `UserConstructionScript`
  (`parent.UserConstructionScript`))