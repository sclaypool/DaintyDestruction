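; BP_Glitter is an enemy-folder projectile that bursts into a growing glitter sphere, then destroys itself.
; A timeline starts half a second after BeginPlay, or earlier through TriggerGrowth, whose Triggered flag prevents the delayed start.
; Each timeline update resizes the collision sphere with overlap updates, activates particles, stops movement, calls an attach and hides the sprite.
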(event `self.ReceiveBeginPlay`
  (`KismetSystemLibrary.Delay` 0.5)
  (if (not (`self.Triggered`))
    (bind (_direction _size) (`Timeline|Timeline_0` :!label _label)
      (:`Update`
        (`SphereComponent.SetSphereRadius` (`self.Sphere`) _size true)
        (`ActorComponent.Activate` (`self.ParticleSystem`) false)
        (`MovementComponent.StopMovementImmediately` (`self.ProjectileMovement`))
        (`self.K2_AttachRootComponentToActor` null)
        (`SceneComponent.SetVisibility` (`self.GlitterSprite`) false false))
      (:`Finished`
        (`self.K2_DestroyActor`)))))

(event `self.ReceiveActorBeginOverlap`
  (params (OtherActor :type "Actor Object Reference")))

(event `self.ReceiveTick`
  (params (DeltaSeconds :type "Float (single-precision)")))

(event `TriggerGrowth`
  (set `self.Triggered` true)
  (goto _label))

(fn `UserConstructionScript`)