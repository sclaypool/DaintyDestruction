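; Paper2D mushroom enemy for a side-scroller that patrols along X, reversing and flipping its flipbook on overlapping BP_TriggerPoint actors.
; Each tick it moves and, while untransformed, spawns BP_Fart when the player is nearby, limited by a delayed-reset cooldown.
; Capsule hits while untransformed can decrease player health.
; After damage, if Transformed is set, it overlaps pawns and plays a flower explosion before switching to another walk flipbook.
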(event `Fart`
  (bind _returnvalue (`SceneComponent.K2_GetComponentLocation` (`self.CapsuleComponent`)))
  (bind (_returnvalue_x _returnvalue_y _returnvalue_z) (`KismetMathLibrary.BreakVector` (- (`self.K2_GetActorLocation` (`GameplayStatics.GetPlayerCharacter` 0)) _returnvalue)))
  ;[1 1 1] Fart Event
  (if (and (not (`self.Farting`)) (not (`self.Transformed`)) (< (`KismetMathLibrary.Abs` _returnvalue_x) 600.0) (< (`KismetMathLibrary.Abs` _returnvalue_z) 200.0))
    (set `self.Farting` true)
    (`|SpawnActorFromClass` "/Game/Blueprints/Enemies/Mushroom/BP_Fart.BP_Fart_C" (`KismetMathLibrary.Conv_VectorToTransform` _returnvalue) "Undefined" "OverrideRootScale")
    (`KismetSystemLibrary.Delay` 10.0)
    (set `self.Farting` false)))

(event `self.ReceiveBeginPlay`)

(event `self.ReceiveActorBeginOverlap`
  (params (OtherActor :type "Actor Object Reference")))

(event `self.ReceiveTick`
  (params (DeltaSeconds :type "Float (single-precision)"))
  (`parent.ReceiveTick` 0.0)
  (`self.Fart`)
  (`self.AddMovementInput` (1.0 0.0 0.0) (* (`self.Rotation`) (`self.My Speed`)) true))

(event `self.Damage`
  (params (AttackType :type "/Game/Blueprints/AttackType Enum" :default "NewEnumerator0"))
  ;[1 1 1] Transform
  (`parent.Damage` AttackType)
  (if (`self.Transformed`)
    (`PrimitiveComponent.SetCollisionResponseToChannel` (`self.CapsuleComponent`) "ECC_Pawn" "ECR_Overlap")
    (`PaperFlipbookComponent.SetFlipbook` (`self.PaperFlipbook`) "/Game/Sprites/Flipbooks/FB_FlowerExplosion.FB_FlowerExplosion")
    (`self.PlayTransformSound`)
    (`SceneComponent.SetRelativeScale3D` (`self.PaperFlipbook`) (1.0 1.0 1.0))
    (`KismetSystemLibrary.Delay` (`PaperFlipbookComponent.GetFlipbookLength` (`self.PaperFlipbook`)))
    (`SceneComponent.SetRelativeScale3D` (`self.PaperFlipbook`) (0.6 0.6 0.6))
    (`PaperFlipbookComponent.SetFlipbook` (`self.PaperFlipbook`) "/Game/Sprites/Flipbooks/GM_walk2.GM_walk2")))

(event `self.CapsuleComponent.OnComponentBeginOverlap`
  (params (OtherActor :type "Actor Object Reference") (OtherComp :type "PrimitiveComponent Object Reference") (OtherBodyIndex :type Integer) (bFromSweep :type Boolean) (SweepResult :type "HitResult Structure (by ref)"))
  ;[1 1 1] Overlap with trigger boundaries
  (cast `/Game/Blueprints/Enemies/Mushroom/BP_TriggerPoint` OtherActor)
  (`self.SetFlipBookMoving` (`self.Rotation`)))

(event `SetFlipBookMoving`
  (params (Rotation :type "Float (double-precision)"))
  ;[1 1 1] Pawn Facing Direction
  (if (> Rotation 0.0)
    (`KismetSystemLibrary.PrintString` "greater than 0")
    (`SceneComponent.K2_SetRelativeRotation` (`self.PaperFlipbook`) (struct :`Yaw` 180.0) false false)
    (set `self.Rotation` -1.0)
    (else
      (`KismetSystemLibrary.PrintString` "less than 0")
      (`SceneComponent.K2_SetRelativeRotation` :`self` (`self.PaperFlipbook`))
      (set `self.Rotation` 1.0))))

(event `self.CapsuleComponent.OnComponentHit`
  (params (OtherActor :type "Actor Object Reference") (OtherComp :type "PrimitiveComponent Object Reference") (NormalImpulse :type "Vector Structure") (Hit :type "HitResult Structure (by ref)"))
  ;[1 1 1] Hit Player
  (if (not (`self.Transformed`))
    (`GameplayStatics.PlaySound2D` null)
    (bind _as2dside_scroller_character (cast `/Game/Blueprints/2DSideScrollerCharacter` OtherActor))
    (if (!= (`PaperFlipbookComponent.GetFlipbook` (`self.PaperFlipbook`)) (`self.GM_Walk2`))
      (`/Game/Blueprints/2DSideScrollerCharacter.Decrease_Health` _as2dside_scroller_character 0.25 false))))

(fn `UserConstructionScript`
  (`parent.UserConstructionScript`))