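; BP_Fart is a short-lived gas hazard in the Mushroom enemy folder that damages the side-scroller player character.
; On BeginPlay it plays a fart sound and destroys itself after three seconds.
; Sphere overlap events track whether the character is in range.
; While in range, Tick repeatedly calls Attack, which lowers player health without knockback, throttled by a Delay and an Attacking flag.
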(event `Attack`
  (if (and (`self.InRange`) (not (`self.Attacking`)))
    (set `self.Attacking` true)
    (bind _as2dside_scroller_character (cast `/Game/Blueprints/2DSideScrollerCharacter` (`GameplayStatics.GetPlayerPawn` 0)))
    (`/Game/Blueprints/2DSideScrollerCharacter.Decrease_Health` _as2dside_scroller_character 0.025 false)
    (`KismetSystemLibrary.Delay` 0.5)
    (set `self.Attacking` false)))

(event `self.ReceiveBeginPlay`
  (`GameplayStatics.SpawnSoundAtLocation` "/Game/Sounds/Fart.Fart" (`self.K2_GetActorLocation`))
  (`KismetSystemLibrary.Delay` 3.0)
  (`self.K2_DestroyActor`))

(event `self.ReceiveActorBeginOverlap`
  (params (OtherActor :type "Actor Object Reference")))

(event `self.ReceiveTick`
  (params (DeltaSeconds :type "Float (single-precision)"))
  (`self.Attack`))

(event `self.Sphere.OnComponentBeginOverlap`
  (params (OtherActor :type "Actor Object Reference") (OtherComp :type "PrimitiveComponent Object Reference") (OtherBodyIndex :type Integer) (bFromSweep :type Boolean) (SweepResult :type "HitResult Structure (by ref)"))
  ;[1 1 1] Check if character is in range
  (cast `/Game/Blueprints/2DSideScrollerCharacter` OtherActor)
  (set `self.InRange` true))

(event `self.Sphere.OnComponentEndOverlap`
  (params (OtherActor :type "Actor Object Reference") (OtherComp :type "PrimitiveComponent Object Reference") (OtherBodyIndex :type Integer))
  ;[1 1 1] Check if character is in range
  (cast `/Game/Blueprints/2DSideScrollerCharacter` OtherActor)
  (set `self.InRange` false))

(fn `UserConstructionScript`)