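; Base enemy for a side-scroller that hurts and knocks back the player on capsule overlap, and becomes Transformed instead of dying.
; Damage subtracts by melee or ranged attack type, hiding the health widget at zero; glitter overlaps trigger growth and Range1 damage.
; Tick updates the health bar and runs passive regen logic, though its timers increment by zero.
; A separate event plays a random transform sound, reaching only two of four options.
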(event `Increase_Health`
  (params (`Heal Amount` :type "Float (double-precision)"))
  (bind _returnvalue (+ (`self.Health`) `Heal Amount`))
  ;[1 1 1] Increase Health
  (if (>= _returnvalue 1.0)
    (set `self.Health` 1.0)
    (else
      (set `self.Health` _returnvalue))))

(event `self.ReceiveBeginPlay`)

(event `PassiveHP`
  (params (Tick :type "Float (double-precision)"))
  (bind _timesinceheal (`self.TimeSinceHeal`))
  ;[1 1 1] Passive HP Regen
  (if (not (`self.Transformed`))
    (bind _output_get (set `self.TimeSinceHit` (+ (`self.TimeSinceHit`) 0.0)))
    (if (>= _output_get 5.0)
      (if (>= _timesinceheal 0.2)
        (`self.Increase_Health` 0.2)
        (set `self.TimeSinceHeal` 0.0)
        (else
          (set `self.TimeSinceHeal` (+ _timesinceheal 0.0)))))))

(event `self.ReceiveActorBeginOverlap`
  (params (OtherActor :type "Actor Object Reference")))

(event `self.ReceiveTick`
  (params (DeltaSeconds :type "Float (single-precision)"))
  ;[1 1 1] HP Bar
  (`self.PassiveHP` DeltaSeconds)
  (bind _asai_health (cast `/Game/Blueprints/Enemies/AI_Health` (`WidgetComponent.GetUserWidgetObject` (`self.Widget`))))
  (`ProgressBar.SetPercent` (`/Game/Blueprints/Enemies/AI_Health.ProgressBar_54` _asai_health) (`self.Health`)))

(event `Damage`
  (params (AttackType :type "/Game/Blueprints/AttackType Enum"))
  (bind _returnvalue (- (`self.Health`) (`self.Range2`)))
  (bind _returnvalue_2 (- (`self.Health`) (`self.Melee2`)))
  (bind _returnvalue_3 (- (`self.Health`) (`self.Range1`)))
  (bind _returnvalue_4 (- (`self.Health`) (`self.Melee1`)))
  ;[1 1 1] Damage
  (if (not (`self.Transformed`))
    (set `self.TimeSinceHit` 0.0)
    (switch `/Game/Blueprints/AttackType` AttackType
      (:`NewEnumerator0`
        (if (<= _returnvalue_4 0.0)
          (set `self.Transformed` true :!label _label)
          (set `self.Health` 0.0)
          (`SceneComponent.SetVisibility` (`self.Widget`) false true)
          (else
            (set `self.Health` _returnvalue_4))))
      (:`NewEnumerator3`
        (if (<= _returnvalue_2 0.0)
          (goto _label)
          (else
            (set `self.Health` _returnvalue_2))))
      (:`NewEnumerator1`
        (if (<= _returnvalue_3 0.0)
          (goto _label)
          (else
            (set `self.Health` _returnvalue_3))))
      (:`NewEnumerator2`
        (if (<= _returnvalue 0.0)
          (goto _label)
          (else
            (set `self.Health` _returnvalue)))))))

(event `PlayTransformSound`
  ;[1 1 1] Transform Sound
  (switch `int` (`KismetMathLibrary.RandomIntegerInRange` 0 1)
    (:`0`
      (`GameplayStatics.PlaySound2D` "/Game/Sounds/Smoochy+Kiss.Smoochy+Kiss"))
    (:`1`
      (`GameplayStatics.PlaySound2D` "/Game/Sounds/POOF.POOF"))
    (:`2`
      (`GameplayStatics.PlaySound2D` "/Game/Sounds/Awww.Awww"))
    (:`3`
      (`GameplayStatics.PlaySound2D` "/Game/Sounds/Sneeze.Sneeze"))))

(event `self.CapsuleComponent.OnComponentBeginOverlap`
  (params (OtherActor :type "Actor Object Reference") (OtherComp :type "PrimitiveComponent Object Reference") (OtherBodyIndex :type Integer) (bFromSweep :type Boolean) (SweepResult :type "HitResult Structure (by ref)"))
  ;[1 1 1] Damage Player
  (if (not (`self.Transformed`))
    (bind _as2dside_scroller_character (cast `/Game/Blueprints/2DSideScrollerCharacter` OtherActor))
    (`/Game/Blueprints/2DSideScrollerCharacter.Decrease_Health` _as2dside_scroller_character (`self.DamageToCharacter`) true)))

(event `self.DamageCapsule.OnComponentBeginOverlap`
  (params (OtherActor :type "Actor Object Reference") (OtherComp :type "PrimitiveComponent Object Reference") (OtherBodyIndex :type Integer) (bFromSweep :type Boolean) (SweepResult :type "HitResult Structure (by ref)"))
  ;[1 1 1] Glitter Attack
  (bind _asbp_glitter (cast `/Game/Blueprints/Enemies/BP_Glitter` OtherActor))
  (`/Game/Blueprints/Enemies/BP_Glitter.TriggerGrowth` _asbp_glitter)
  (if (not (`self.Transformed`))
    (`self.Damage` "NewEnumerator1")))

(fn `UserConstructionScript`)