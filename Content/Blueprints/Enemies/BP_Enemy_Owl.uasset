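; Owl enemy for a 2D side-scroller that fires lasers at the player until it is transformed.
; LaserBox overlap flags the player in range, and Tick spawns BP_Laser from the Eye aimed at them, using the shoot flipbook's length as cooldown.
; Damage calls the parent, then plays a hit animation or, if Transformed, a flower explosion into an idle with pawn overlap.
; The construction script orients the sprite from Rotation.
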(event `self.ReceiveBeginPlay`)

(event `self.ReceiveActorBeginOverlap`
  (params (OtherActor :type "Actor Object Reference")))

(event `self.ReceiveTick`
  (params (DeltaSeconds :type "Float (single-precision)"))
  (`parent.ReceiveTick` 0.0)
  (`self.Shoot`))

(event `self.Laser Box.OnComponentBeginOverlap`
  (params (OtherActor :type "Actor Object Reference") (OtherComp :type "PrimitiveComponent Object Reference") (OtherBodyIndex :type Integer) (bFromSweep :type Boolean) (SweepResult :type "HitResult Structure (by ref)"))
  ;[1 1 1] Player in Range?
  (cast `/Game/Blueprints/2DSideScrollerCharacter` OtherActor)
  (set `self.Inside` true))

(event `self.Laser Box.OnComponentEndOverlap`
  (params (OtherActor :type "Actor Object Reference") (OtherComp :type "PrimitiveComponent Object Reference") (OtherBodyIndex :type Integer))
  ;[1 1 1] Player in Range?
  (cast `/Game/Blueprints/2DSideScrollerCharacter` OtherActor)
  (set `self.Inside` false))

(event `self.Damage`
  (params (AttackType :type "/Game/Blueprints/AttackType Enum" :default "NewEnumerator0"))
  ;[1 1 1] Process Owl Damage
  (`parent.Damage` AttackType)
  (if (`self.Transformed`)
    (`PrimitiveComponent.SetCollisionResponseToChannel` (`self.CapsuleComponent`) "ECC_Pawn" "ECR_Overlap")
    (`PaperFlipbookComponent.SetFlipbook` (`self.PaperFlipbook`) "/Game/Sprites/Flipbooks/FB_FlowerExplosion.FB_FlowerExplosion")
    (`self.PlayTransformSound`)
    (`SceneComponent.SetRelativeScale3D` (`self.PaperFlipbook`) (1.0 1.0 1.0))
    (`KismetSystemLibrary.Delay` (`PaperFlipbookComponent.GetFlipbookLength` (`self.PaperFlipbook`)))
    (`SceneComponent.SetRelativeScale3D` (`self.PaperFlipbook`) (0.45 0.45 0.45))
    (`PaperFlipbookComponent.SetFlipbook` (`self.PaperFlipbook`) "/Game/Sprites/Flipbooks/GO_Idle2.GO_Idle2")
    (else
      (`PaperFlipbookComponent.SetFlipbook` (`self.PaperFlipbook`) "/Game/Sprites/Flipbooks/FB_Owl_Evil_Hit.FB_Owl_Evil_Hit")
      (`KismetSystemLibrary.Delay` (`PaperFlipbookComponent.GetFlipbookLength` (`self.PaperFlipbook`)))
      (if (`self.Transformed`)
        (`PaperFlipbookComponent.SetFlipbook` (`self.PaperFlipbook`) "/Game/Sprites/Flipbooks/GO_Idle2.GO_Idle2")
        (else
          (`PaperFlipbookComponent.SetFlipbook` (`self.PaperFlipbook`) "/Game/Sprites/Flipbooks/FB_Owl_Evil_Idle.FB_Owl_Evil_Idle"))))))

(event `Shoot`
  (bind _returnvalue (`SceneComponent.K2_GetComponentLocation` (`self.Eye`)))
  ;[1 1 1] Shoot at Player
  (if (and (`self.Inside`) (not (`self.Shooting`)) (not (`self.Transformed`)))
    (set `self.Shooting` true)
    (bind _as2dside_scroller_character (cast `/Game/Blueprints/2DSideScrollerCharacter` (`GameplayStatics.GetPlayerPawn` 0)))
    (`PaperFlipbookComponent.SetFlipbook` (`self.PaperFlipbook`) "/Game/Sprites/Flipbooks/FB_Owl_Evil_Shoot.FB_Owl_Evil_Shoot")
    (`|SpawnActorFromClass` "/Game/Blueprints/Enemies/BP_Laser.BP_Laser_C" (`KismetMathLibrary.MakeTransform` _returnvalue (`KismetMathLibrary.FindLookAtRotation` _returnvalue (`self.K2_GetActorLocation` _as2dside_scroller_character))) "Undefined" "OverrideRootScale")
    (`KismetSystemLibrary.Delay` (`PaperFlipbookComponent.GetFlipbookLength` (`self.PaperFlipbook`)))
    (set `self.Shooting` false)
    (if (not (`self.Transformed`))
      (`PaperFlipbookComponent.SetFlipbook` (`self.PaperFlipbook`) "/Game/Sprites/Flipbooks/FB_Owl_Evil_Idle.FB_Owl_Evil_Idle")
      (else
        (`PaperFlipbookComponent.SetFlipbook` (`self.PaperFlipbook`) "/Game/Sprites/Flipbooks/GO_Idle2.GO_Idle2")))))

(fn `UserConstructionScript`
  (`parent.UserConstructionScript`)
  (if (> (`self.Rotation`) 0.0)
    (`SceneComponent.K2_SetRelativeRotation` (`self.PaperFlipbook`) (struct :`Yaw` 180.0) false false)
    (else
      (`SceneComponent.K2_SetRelativeRotation` :`self` (`self.PaperFlipbook`)))))