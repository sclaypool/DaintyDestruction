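; Boss enemy for the 2D side-scroller that attacks the player and triggers the game win when damaged while Transformed.
; While the player is inside AttackBox, Tick starts a random attack: blood rain spawned overhead or lightning that directly reduces health.
; Flipbook lengths time each attack and cooldown, and a beam particle tracks the player.
; Rotator overlaps flip the sprite toward the player.
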(event `Attack`
  (bind _returnvalue (`GameplayStatics.GetPlayerPawn` 0))
  (bind _paperflipbook (`self.PaperFlipbook`))
  (bind _paperflipbook_2 (`self.PaperFlipbook`))
  (bind _paperflipbook_3 (`self.PaperFlipbook`))
  (bind _paperflipbook_4 (`self.PaperFlipbook`))
  (bind _returnvalue_2 (/ (`PaperFlipbookComponent.GetFlipbookLength` _paperflipbook) 2.0))
  (bind _returnvalue_3 (/ (`PaperFlipbookComponent.GetFlipbookLength` _paperflipbook_4) 2.0))
  ;[1 1 1] Attack the Character
  (if (and (`self.InRange`) (not (`self.Attacking`)))
    (set `self.Attacking` true)
    (switch `int` (`KismetMathLibrary.RandomIntegerInRange` 0 1)
      (:`0`
        (`PaperFlipbookComponent.SetFlipbook` _paperflipbook_4 "/Game/Sprites/Flipbooks/AntiChar_AttackUp_Anim.AntiChar_AttackUp_Anim")
        (`GameplayStatics.PlaySound2D` "/Game/Sounds/EvilLaugh.EvilLaugh")
        (`KismetSystemLibrary.Delay` _returnvalue_3)
        (`|SpawnActorFromClass` "/Game/Blueprints/Enemies/Boss/BP_BloodRain.BP_BloodRain_C" (`KismetMathLibrary.MakeTransform` (+ (`self.K2_GetActorLocation` _returnvalue) (0.0 0.0 500.0))) "Undefined" "OverrideRootScale")
        (`KismetSystemLibrary.Delay` _returnvalue_3)
        (`PaperFlipbookComponent.SetFlipbook` _paperflipbook_3 "/Game/Sprites/Flipbooks/AntiChar_Idle_Anim.AntiChar_Idle_Anim")
        (`KismetSystemLibrary.Delay` (* (`PaperFlipbookComponent.GetFlipbookLength` _paperflipbook_3) 3.0))
        (set `self.Attacking` false))
      (:`1`
        (bind _as2dside_scroller_character (cast `/Game/Blueprints/2DSideScrollerCharacter` _returnvalue)
          (:`then`
            (`GameplayStatics.PlaySound2D` "/Game/Sounds/EvilLaugh.EvilLaugh")
            (`/Game/Blueprints/2DSideScrollerCharacter.Decrease_Health` _as2dside_scroller_character 0.05 false)
            (`PaperFlipbookComponent.SetFlipbook` _paperflipbook "/Game/Sprites/Flipbooks/AntiChar_AttackDown_Anim.AntiChar_AttackDown_Anim")
            (`KismetSystemLibrary.Delay` _returnvalue_2)
            (`SceneComponent.SetVisibility` (`self.ParticleSystem`) true false)
            (`KismetSystemLibrary.Delay` _returnvalue_2)
            (`SceneComponent.SetVisibility` (`self.ParticleSystem`) false false)
            (`PaperFlipbookComponent.SetFlipbook` _paperflipbook_2 "/Game/Sprites/Flipbooks/AntiChar_Idle_Anim.AntiChar_Idle_Anim")
            (`KismetSystemLibrary.Delay` (* (`PaperFlipbookComponent.GetFlipbookLength` _paperflipbook_2) 3.0))
            (set `self.Attacking` false))
          (:`CastFailed`
            (set `self.Attacking` false)))))))

(event `self.ReceiveBeginPlay`)

(event `self.ReceiveActorBeginOverlap`
  (params (OtherActor :type "Actor Object Reference")))

(event `self.ReceiveTick`
  (params (DeltaSeconds :type "Float (single-precision)"))
  (bind _particlesystem (`self.ParticleSystem`))
  (`parent.ReceiveTick` 0.0)
  (`self.Attack`)
  ;[1 1 1] Make sure the lightning is following the character
  (if (`self.InRange`)
    (`ParticleSystemComponent.SetBeamTargetPoint` _particlesystem 0 (`self.K2_GetActorLocation` (`GameplayStatics.GetPlayerPawn` 0)) 0)
    (`ParticleSystemComponent.SetBeamSourcePoint` _particlesystem 0 (`SceneComponent.K2_GetComponentLocation` (`self.ParticleSystem`)) 0)))

(event `self.Damage`
  (params (AttackType :type "/Game/Blueprints/AttackType Enum" :default "NewEnumerator0"))
  ;[1 1 1] Take Damage and die
  (`parent.Damage` AttackType)
  (if (`self.Transformed`)
    (bind _as2dside_scroller_character (cast `/Game/Blueprints/2DSideScrollerCharacter` (`GameplayStatics.GetPlayerPawn` 0)))
    (`/Game/Blueprints/2DSideScrollerCharacter.WinGame` _as2dside_scroller_character)
    (`self.K2_DestroyActor`)))

(event `self.Rotator.OnComponentBeginOverlap`
  (params (OtherActor :type "Actor Object Reference") (OtherComp :type "PrimitiveComponent Object Reference") (OtherBodyIndex :type Integer) (bFromSweep :type Boolean) (SweepResult :type "HitResult Structure (by ref)"))
  (bind _returnvalue_x (`KismetMathLibrary.BreakVector` (`self.K2_GetActorLocation`)))
  ;[1 1 1] Change Rotation
  (bind _as2dside_scroller_character (cast `/Game/Blueprints/2DSideScrollerCharacter` OtherActor))
  (bind _returnvalue_x_2 (`KismetMathLibrary.BreakVector` (`self.K2_GetActorLocation` _as2dside_scroller_character)))
  (bind _returnvalue_x_3 (`KismetMathLibrary.BreakVector` (`self.K2_GetActorLocation` (stale `self.Rotator.OnComponentEndOverlap` _as2dside_scroller_character))))
  (if (or (> _returnvalue_x_2 _returnvalue_x) (> _returnvalue_x_3 _returnvalue_x)) :!label _label
    (set `self.Rotation` 1.0)
    (`SceneComponent.K2_SetRelativeRotation` :`self` (`self.PaperFlipbook`))
    (else
      (set `self.Rotation` -1.0)
      (`SceneComponent.K2_SetRelativeRotation` (`self.PaperFlipbook`) (struct :`Yaw` 180.0) false false))))

(event `self.Rotator.OnComponentEndOverlap`
  (params (OtherActor :type "Actor Object Reference") (OtherComp :type "PrimitiveComponent Object Reference") (OtherBodyIndex :type Integer))
  ;[1 1 1] Change Rotation
  (bind _as2dside_scroller_character (cast `/Game/Blueprints/2DSideScrollerCharacter` OtherActor))
  (goto _label))

(event `self.AttackBox.OnComponentBeginOverlap`
  (params (OtherActor :type "Actor Object Reference") (OtherComp :type "PrimitiveComponent Object Reference") (OtherBodyIndex :type Integer) (bFromSweep :type Boolean) (SweepResult :type "HitResult Structure (by ref)"))
  ;[1 1 1] Verify Character is in range
  (cast `/Game/Blueprints/2DSideScrollerCharacter` OtherActor)
  (set `self.InRange` true))

(event `self.AttackBox.OnComponentEndOverlap`
  (params (OtherActor :type "Actor Object Reference") (OtherComp :type "PrimitiveComponent Object Reference") (OtherBodyIndex :type Integer))
  ;[1 1 1] Verify Character is in range
  (cast `/Game/Blueprints/2DSideScrollerCharacter` OtherActor)
  (set `self.InRange` false))

(fn `UserConstructionScript`
  (`parent.UserConstructionScript`)
  (if (< (`self.Rotation`) 0.0)
    (`SceneComponent.K2_SetRelativeRotation` (`self.PaperFlipbook`) (struct :`Yaw` 180.0) false false)
    (else
      (`SceneComponent.K2_SetRelativeRotation` :`self` (`self.PaperFlipbook`)))))