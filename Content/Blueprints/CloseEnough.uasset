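; CloseEnough is a behavior tree decorator for the frog AI that gates a branch on distance to the actor it follows.
; It caches the owning Frog_AI_CON and compares its pawn's location with that of the TargetToFollow blackboard actor.
; Despite the name, the check passes when the distance is at least AcceptableDistance, so it is true while the frog is not yet close.
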(fn `PerformConditionCheck`
  (params (OwnerActor :type "Actor Object Reference"))
  (returns (ReturnValue :type Boolean))
  (bind _asfrog_ai_con (cast `/Game/Blueprints/Frog_AI_CON` OwnerActor)
    (:`then`
      (set `self.AI_CON_Ref` _asfrog_ai_con))
    (:`CastFailed`
      _))
  (return (>= (`KismetMathLibrary.VSize` (- (`Actor.K2_GetActorLocation` (`BTFunctionLibrary.GetBlackboardValueAsActor` (`self.TargetToFollow`))) (`Actor.K2_GetActorLocation` (`Controller.K2_GetPawn` (`self.AI_CON_Ref`))))) (`self.AcceptableDistance`))))