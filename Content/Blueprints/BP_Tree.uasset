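; Evil tree enemy for a 2D side-scroller that swipes at the player from its left or right side.
; Per-side trigger volumes play a swipe flipbook, then return to idle; a half-length Delay opens the Attacking window mid-animation.
; During that window, Tick damages the player inside the matching damage volume and clears the flags to end the hit.
; Hit-reaction and death logic exists but is disconnected, so the tree ignores damage.
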(event `ChangeAnimation`
  (params (Flipbook :type "PaperFlipbook Object Reference"))
  (bind _paperflipbook (`self.PaperFlipbook`))
  (`PaperFlipbookComponent.SetFlipbook` _paperflipbook Flipbook)
  (`KismetSystemLibrary.Delay` (`PaperFlipbookComponent.GetFlipbookLength` _paperflipbook))
  (`PaperFlipbookComponent.SetFlipbook` _paperflipbook "/Game/Sprites/Flipbooks/FB_Tree_Evil_Idle.FB_Tree_Evil_Idle"))

(event `self.ReceiveBeginPlay`)

(event `self.ReceiveActorBeginOverlap`
  (params (OtherActor :type "Actor Object Reference")))

(event `self.ReceiveTick`
  (params (DeltaSeconds :type "Float (single-precision)"))
  (if (`self.Attacking`)
    (if (`self.LeftAttack`)
      (for _array_element (`PrimitiveComponent.GetOverlappingActors` (`self.LeftDamage`) null)
        (bind _as2dside_scroller_character (cast `/Game/Blueprints/2DSideScrollerCharacter` _array_element))
        (`/Game/Blueprints/2DSideScrollerCharacter.Decrease_Health` _as2dside_scroller_character 0.1)
        (`KismetSystemLibrary.PrintString` "Left Attack")
        (set `self.Attacking` false)
        (set `self.LeftTriggered` false)
        (set `self.LeftAttack` false))
      (elif (`self.RightAttack`)
        (for _array_element_2 (`PrimitiveComponent.GetOverlappingActors` (`self.RightDamage`) null)
          (bind _as2dside_scroller_character_2 (cast `/Game/Blueprints/2DSideScrollerCharacter` _array_element_2))
          (`/Game/Blueprints/2DSideScrollerCharacter.Decrease_Health` _as2dside_scroller_character_2 0.1)
          (`KismetSystemLibrary.PrintString` "Right Attack")
          (set `self.Attacking` false)
          (set `self.RightTriggered` false)
          (set `self.RightAttack` false))))))

(event `self.LeftTrigger.OnComponentBeginOverlap`
  (params (OtherActor :type "Actor Object Reference") (OtherComp :type "PrimitiveComponent Object Reference") (OtherBodyIndex :type Integer) (bFromSweep :type Boolean) (SweepResult :type "HitResult Structure (by ref)"))
  (bind _returnvalue (/ (`PaperFlipbookComponent.GetFlipbookLength` (`self.PaperFlipbook`)) 2.0))
  ;[1 1 1] Left Attack
  (cast `/Game/Blueprints/2DSideScrollerCharacter` OtherActor)
  (if (and (not (`self.Attacking`)) (not (`self.LeftTriggered`)))
    (set `self.LeftTriggered` true)
    (`self.ChangeAnimation` "/Game/Sprites/Flipbooks/FB_Tree_Evil_Swipe_Left.FB_Tree_Evil_Swipe_Left")
    (`KismetSystemLibrary.Delay` _returnvalue)
    (set `self.Attacking` true)
    (`KismetSystemLibrary.Delay` _returnvalue)
    (set `self.Attacking` false)))

(event `self.LeftDamage.OnComponentBeginOverlap`
  (params (OtherActor :type "Actor Object Reference") (OtherComp :type "PrimitiveComponent Object Reference") (OtherBodyIndex :type Integer) (bFromSweep :type Boolean) (SweepResult :type "HitResult Structure (by ref)"))
  ;[1 1 1] Left Attack
  (cast `/Game/Blueprints/2DSideScrollerCharacter` OtherActor)
  (set `self.LeftAttack` true))

(event `self.ReceiveAnyDamage`
  (params (Damage :type "Float (single-precision)") (DamageType :type "DamageType Object Reference") (InstigatedBy :type "Controller Object Reference") (DamageCauser :type "Actor Object Reference")))

(event `self.LeftTrigger.OnComponentEndOverlap`
  (params (OtherActor :type "Actor Object Reference") (OtherComp :type "PrimitiveComponent Object Reference") (OtherBodyIndex :type Integer))
  ;[1 1 1] Left Attack
  (cast `/Game/Blueprints/2DSideScrollerCharacter` OtherActor)
  (if (not (`self.Attacking`))
    (set `self.LeftTriggered` false)))

(event `self.LeftDamage.OnComponentEndOverlap`
  (params (OtherActor :type "Actor Object Reference") (OtherComp :type "PrimitiveComponent Object Reference") (OtherBodyIndex :type Integer))
  ;[1 1 1] Left Attack
  (cast `/Game/Blueprints/2DSideScrollerCharacter` OtherActor)
  (set `self.LeftAttack` false))

(event `self.RightTrigger.OnComponentBeginOverlap`
  (params (OtherActor :type "Actor Object Reference") (OtherComp :type "PrimitiveComponent Object Reference") (OtherBodyIndex :type Integer) (bFromSweep :type Boolean) (SweepResult :type "HitResult Structure (by ref)"))
  (bind _returnvalue (/ (`PaperFlipbookComponent.GetFlipbookLength` (`self.PaperFlipbook`)) 2.0))
  ;[1 1 1] Right Attack
  (cast `/Game/Blueprints/2DSideScrollerCharacter` OtherActor)
  (if (and (not (`self.Attacking`)) (not (`self.RightTriggered`)))
    (set `self.RightTriggered` true)
    (`self.ChangeAnimation` "/Game/Sprites/Flipbooks/FB_Tree_Evil_Swipe_Right.FB_Tree_Evil_Swipe_Right")
    (`KismetSystemLibrary.Delay` _returnvalue)
    (set `self.Attacking` true)
    (`KismetSystemLibrary.Delay` _returnvalue)
    (set `self.Attacking` false)))

(event `self.RightDamage.OnComponentBeginOverlap`
  (params (OtherActor :type "Actor Object Reference") (OtherComp :type "PrimitiveComponent Object Reference") (OtherBodyIndex :type Integer) (bFromSweep :type Boolean) (SweepResult :type "HitResult Structure (by ref)"))
  ;[1 1 1] Right Attack
  (cast `/Game/Blueprints/2DSideScrollerCharacter` OtherActor)
  (set `self.RightAttack` true))

(event `self.RightTrigger.OnComponentEndOverlap`
  (params (OtherActor :type "Actor Object Reference") (OtherComp :type "PrimitiveComponent Object Reference") (OtherBodyIndex :type Integer))
  ;[1 1 1] Right Attack
  (cast `/Game/Blueprints/2DSideScrollerCharacter` OtherActor)
  (set `self.RightTriggered` false))

(event `self.RightDamage.OnComponentEndOverlap`
  (params (OtherActor :type "Actor Object Reference") (OtherComp :type "PrimitiveComponent Object Reference") (OtherBodyIndex :type Integer))
  ;[1 1 1] Right Attack
  (cast `/Game/Blueprints/2DSideScrollerCharacter` OtherActor)
  (set `self.RightAttack` false))

(fn `UserConstructionScript`)