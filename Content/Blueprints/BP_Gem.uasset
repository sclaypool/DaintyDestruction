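; Collectible 2D gem that raises the side-scroller character's gem count and restores either mana or health, chosen by a flag.
; The GemBounce timeline, played from Tick, animates it by adding local offsets.
; Box overlap with the character triggers the reward behind a one-shot CanIncrease guard.
; The flipbook then switches to a pop animation, and the actor destroys itself after that animation's duration.
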(event `self.ReceiveBeginPlay`
  (`PaperFlipbookComponent.SetFlipbook` (`self.PaperFlipbook`) (`self.Default_Flipbook`)))

(event `self.ReceiveActorBeginOverlap`
  (params (OtherActor :type "Actor Object Reference")))

(event `self.ReceiveTick`
  (params (DeltaSeconds :type "Float (single-precision)"))
  (bind (_direction _gem) (`Timeline|GemBounce`)
    (:`Update`
      (`self.K2_AddActorLocalOffset` _gem))))

(event `self.Box.OnComponentBeginOverlap`
  (params (OtherActor :type "Actor Object Reference") (OtherComp :type "PrimitiveComponent Object Reference") (OtherBodyIndex :type Integer) (bFromSweep :type Boolean) (SweepResult :type "HitResult Structure (by ref)"))
  (bind _pop_flipbook (`self.Pop_Flipbook`))
  (bind _hpormpgain (`self.HPorMPGain`))
  (bind _as2dside_scroller_character (cast `/Game/Blueprints/2DSideScrollerCharacter` OtherActor))
  (if (`self.CanIncrease`)
    (`/Game/Blueprints/2DSideScrollerCharacter.Increase_Gem` _as2dside_scroller_character)
    (set `self.CanIncrease` false)
    (if (`self.ManaGem`)
      (`/Game/Blueprints/2DSideScrollerCharacter.Increase_Mana` _as2dside_scroller_character _hpormpgain)
      (else
        (`/Game/Blueprints/2DSideScrollerCharacter.Increase_Health` _as2dside_scroller_character _hpormpgain)))
    (`PaperFlipbookComponent.SetFlipbook` (`self.PaperFlipbook`) _pop_flipbook)
    (`KismetSystemLibrary.Delay` (`PaperFlipbook.GetTotalDuration` _pop_flipbook))
    (`self.K2_DestroyActor`)))

(fn `UserConstructionScript`)