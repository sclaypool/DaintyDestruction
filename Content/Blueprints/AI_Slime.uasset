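; Paper2D slime enemy for a side-scroller that hops while idle and hurts the player on contact.
; Left and right trigger volumes set its facing and make it move toward the player, otherwise landing schedules the next, usually reversed, hop.
; Projectile overlaps apply damage.
; At zero health it transforms via a flower explosion into a harmless, rescaled walker that stops hopping but still follows the player.
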(event `self.ReceiveBeginPlay`)

(event `self.ReceiveActorBeginOverlap`
  (params (OtherActor :type "Actor Object Reference")))

(event `self.ReceiveTick`
  (params (DeltaSeconds :type "Float (single-precision)"))
  (if (or (`self.LeftTriggered`) (`self.RightTriggered`))
    (`self.AddMovementInput` (1.0 0.0 0.0) (* (`self.Rotation`) (`self.MySpeed`)) true)
    (elif (and (`self.Idle`) (not (`self.Jiggle`)) (not (`self.Transformed`)))
      (set `self.Idle` false)
      (set `self.Jiggle` true)
      (`PaperFlipbookComponent.SetFlipbook` (`self.PaperFlipbook`) "/Game/Sprites/Flipbooks/ES_jiggle2.ES_jiggle2")
      (`self.LaunchCharacter` (`KismetMathLibrary.MakeVector` (* (`self.Rotation`) -200.0) 0.0 200.0))
      (elif (`self.Transformed`)
        _))))

(event `self.OnLanded`
  (params (Hit :type "HitResult Structure (by ref)"))
  ;[1 1 1] Slime Jiggle/Jump
  (set `self.Jiggle` false)
  (`PaperFlipbookComponent.SetFlipbook` (`self.PaperFlipbook`) "/Game/Sprites/Flipbooks/ES_Idle.ES_Idle")
  (if (> (`self.Rotation`) 0.0)
    (`SceneComponent.K2_SetRelativeRotation` (`self.PaperFlipbook`) (struct) false false)
    (else
      (`SceneComponent.K2_SetRelativeRotation` (`self.PaperFlipbook`) (struct :`Yaw` 180.0) false false)))
  (`KismetSystemLibrary.Delay` (* (`PaperFlipbookComponent.GetFlipbookLength` (`self.PaperFlipbook`)) 2.0))
  (if (and (not (`self.LeftTriggered`)) (not (`self.RightTriggered`)))
    (set `self.Rotation` (* (`self.Rotation`) -1.0)))
  (set `self.Idle` true))

(event `self.Left Trigger.OnComponentBeginOverlap`
  (params (OtherActor :type "Actor Object Reference") (OtherComp :type "PrimitiveComponent Object Reference") (OtherBodyIndex :type Integer) (bFromSweep :type Boolean) (SweepResult :type "HitResult Structure (by ref)"))
  ;[1 1 1] Left Overlap
  (cast `/Game/Blueprints/2DSideScrollerCharacter` OtherActor)
  (set `self.LeftTriggered` true)
  (`SceneComponent.K2_SetRelativeRotation` (`self.PaperFlipbook`) (struct :`Yaw` 180.0) false false)
  (set `self.Rotation` -1.0)
  (if (`self.Transformed`)
    (`PaperFlipbookComponent.SetFlipbook` (`self.PaperFlipbook`) "/Game/Sprites/Flipbooks/GT_walk2.GT_walk2")))

(event `self.Left Trigger.OnComponentEndOverlap`
  (params (OtherActor :type "Actor Object Reference") (OtherComp :type "PrimitiveComponent Object Reference") (OtherBodyIndex :type Integer))
  ;[1 1 1] Left Overlap
  (cast `/Game/Blueprints/2DSideScrollerCharacter` OtherActor)
  (set `self.LeftTriggered` false)
  (if (`self.Transformed`)
    (`PaperFlipbookComponent.SetFlipbook` (`self.PaperFlipbook`) "/Game/Sprites/Flipbooks/GT_idle2.GT_idle2")))

(event `self.Right Trigger.OnComponentBeginOverlap`
  (params (OtherActor :type "Actor Object Reference") (OtherComp :type "PrimitiveComponent Object Reference") (OtherBodyIndex :type Integer) (bFromSweep :type Boolean) (SweepResult :type "HitResult Structure (by ref)"))
  ;[1 1 1] Right Overlap
  (cast `/Game/Blueprints/2DSideScrollerCharacter` OtherActor)
  (set `self.RightTriggered` true)
  (`SceneComponent.K2_SetRelativeRotation` :`self` (`self.PaperFlipbook`))
  (set `self.Rotation` 1.0)
  (if (`self.Transformed`)
    (`PaperFlipbookComponent.SetFlipbook` (`self.PaperFlipbook`) "/Game/Sprites/Flipbooks/GT_walk2.GT_walk2")))

(event `self.Right Trigger.OnComponentEndOverlap`
  (params (OtherActor :type "Actor Object Reference") (OtherComp :type "PrimitiveComponent Object Reference") (OtherBodyIndex :type Integer))
  ;[1 1 1] Right Overlap
  (cast `/Game/Blueprints/2DSideScrollerCharacter` OtherActor)
  (set `self.RightTriggered` false)
  (if (`self.Transformed`)
    (`PaperFlipbookComponent.SetFlipbook` (`self.PaperFlipbook`) "/Game/Sprites/Flipbooks/GT_idle2.GT_idle2")))

(event `self.ReceiveAnyDamage`
  (params (Damage :type "Float (single-precision)") (DamageType :type "DamageType Object Reference") (InstigatedBy :type "Controller Object Reference") (DamageCauser :type "Actor Object Reference"))
  (bind _returnvalue (- (`self.Health`) Damage))
  ;[1 1 1] Process Slime Damage
  (`KismetSystemLibrary.PrintString` "received damage")
  (if (<= _returnvalue 0.0)
    (set `self.Transformed` true)
    (`KismetSystemLibrary.PrintString` "died")
    (set `self.Health` 0.0)
    (`PaperFlipbookComponent.SetFlipbook` (`self.PaperFlipbook`) "/Game/Sprites/Flipbooks/FB_FlowerExplosion.FB_FlowerExplosion")
    (`GameplayStatics.PlaySound2D` "/Game/Sounds/Smoochy+Kiss.Smoochy+Kiss")
    (`KismetSystemLibrary.Delay` (`PaperFlipbookComponent.GetFlipbookLength` (`self.PaperFlipbook`)))
    (`SceneComponent.SetRelativeScale3D` (`self.PaperFlipbook`) (0.6 0.6 0.6))
    (`PaperFlipbookComponent.SetFlipbook` (`self.PaperFlipbook`) "/Game/Sprites/Flipbooks/GT_walk2.GT_walk2")
    (`PrimitiveComponent.SetCollisionEnabled` (`self.CapsuleComponent`) "QueryOnly")
    (else
      (set `self.Health` _returnvalue)
      (`PaperFlipbookComponent.SetFlipbook` (`self.PaperFlipbook`) "/Game/Sprites/Flipbooks/ES_hit2.ES_hit2")
      (`KismetSystemLibrary.Delay` (`PaperFlipbookComponent.GetFlipbookLength` (`self.PaperFlipbook`)))
      (if (`self.Transformed`)
        (`PaperFlipbookComponent.SetFlipbook` (`self.PaperFlipbook`) "/Game/Sprites/Flipbooks/GT_walk2.GT_walk2")
        (else
          (`PaperFlipbookComponent.SetFlipbook` (`self.PaperFlipbook`) "/Game/Sprites/Flipbooks/ES_jiggle2.ES_jiggle2"))))))

(event `self.CapsuleComponent.OnComponentHit`
  (params (OtherActor :type "Actor Object Reference") (OtherComp :type "PrimitiveComponent Object Reference") (NormalImpulse :type "Vector Structure") (Hit :type "HitResult Structure (by ref)"))
  ;[1 1 1] Process damage to 2D character
  (bind _as2dside_scroller_character (cast `/Game/Blueprints/2DSideScrollerCharacter` OtherActor))
  (if (not (`self.Transformed`))
    (`/Game/Blueprints/2DSideScrollerCharacter.Decrease_Health` _as2dside_scroller_character 0.25)))

(event `self.DamageCapsule.OnComponentBeginOverlap`
  (params (OtherActor :type "Actor Object Reference") (OtherComp :type "PrimitiveComponent Object Reference") (OtherBodyIndex :type Integer) (bFromSweep :type Boolean) (SweepResult :type "HitResult Structure (by ref)"))
  ;[1 1 1] Process damage to slime from long range attack
  (bind _asbp_projectile (cast `/Game/Blueprints/BP_Projectile` OtherActor))
  (`PrimitiveComponent.SetCollisionEnabled` (`/Game/Blueprints/BP_Projectile.Sphere` _asbp_projectile) "NoCollision")
  (`GameplayStatics.ApplyDamage` self 0.2 null _asbp_projectile))

(event `Increase_Health`
  (params (`Heal Amount` :type "Float (double-precision)"))
  (bind _returnvalue (+ (`self.Health`) `Heal Amount`))
  (if (>= _returnvalue 1.0)
    (set `self.Health` 1.0)
    (else
      (set `self.Health` _returnvalue))))

(fn `UserConstructionScript`)