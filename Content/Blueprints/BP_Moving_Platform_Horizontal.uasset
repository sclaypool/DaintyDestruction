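; BP_Moving_Platform_Horizontal is a Paper2D moving platform that can change to a "good" appearance.
; Tick plays the MoveHorizontal timeline, whose track value is added as a local offset on each update, without sweep.
; While Transformed is false, overlapping the Transform component clears ParticleSystem, swaps the flipbook to FB_Platform_Moving_Good and shifts it along local Y.
; This graph never sets Transformed itself.
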(event `self.ReceiveBeginPlay`)

(event `self.ReceiveActorBeginOverlap`
  (params (OtherActor :type "Actor Object Reference")))

(event `self.ReceiveTick`
  (params (DeltaSeconds :type "Float (single-precision)"))
  (bind (_direction _newtrack_0) (`Timeline|MoveHorizontal`)
    (:`Update`
      (`self.K2_AddActorLocalOffset` _newtrack_0))))

(event `self.Transform.OnComponentBeginOverlap`
  (params (OtherActor :type "Actor Object Reference") (OtherComp :type "PrimitiveComponent Object Reference") (OtherBodyIndex :type Integer) (bFromSweep :type Boolean) (SweepResult :type "HitResult Structure (by ref)"))
  (if (not (`self.Transformed`))
    (set `self.ParticleSystem` null)
    (`PaperFlipbookComponent.SetFlipbook` (`self.PaperFlipbook`) "/Game/Sprites/Flipbooks/FB_Platform_Moving_Good.FB_Platform_Moving_Good")
    (`SceneComponent.K2_AddLocalOffset` (`self.PaperFlipbook`) (0.0 -40.0 0.0) false false)))

(fn `UserConstructionScript`)