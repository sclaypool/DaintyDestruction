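; BP_Easter_Egg is a polka-dot egg actor, kept in the Deprecated folder, that reacts when the side-scroller character touches it.
; A Box overlap with that character switches the Paper2D flipbook to a transition animation, waits for its length, then shows the "good" egg flipbook.
; The Rise timeline then moves the egg by per-update local offsets and destroys it on finish, with no score or reward logic.
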(event `self.ReceiveBeginPlay`)

(event `self.ReceiveActorBeginOverlap`
  (params (OtherActor :type "Actor Object Reference")))

(event `self.ReceiveTick`
  (params (DeltaSeconds :type "Float (single-precision)")))

(event `self.Box.OnComponentBeginOverlap`
  (params (OtherActor :type "Actor Object Reference") (OtherComp :type "PrimitiveComponent Object Reference") (OtherBodyIndex :type Integer) (bFromSweep :type Boolean) (SweepResult :type "HitResult Structure (by ref)"))
  (cast `/Game/Blueprints/2DSideScrollerCharacter` OtherActor)
  (`PaperFlipbookComponent.SetFlipbook` (`self.PaperFlipbook`) "/Game/Sprites/Flipbooks/FB_Egg_Polka_Transition.FB_Egg_Polka_Transition")
  (`KismetSystemLibrary.Delay` (`PaperFlipbookComponent.GetFlipbookLength` (`self.PaperFlipbook`)))
  (`PaperFlipbookComponent.SetFlipbook` (`self.PaperFlipbook`) "/Game/Sprites/Flipbooks/FB_Egg_Polka_Good.FB_Egg_Polka_Good")
  (bind (_direction _newtrack_0) (`Timeline|Rise` :!via `PlayFromStart`)
    (:`Update`
      (`self.K2_AddActorLocalOffset` _newtrack_0))
    (:`Finished`
      (`self.K2_DestroyActor`))))

(fn `UserConstructionScript`)