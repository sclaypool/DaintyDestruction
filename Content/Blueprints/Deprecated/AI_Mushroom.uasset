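; Side-scroller mushroom enemy that patrols between BP_TriggerPoint volumes, hurts the player on contact and periodically spawns BP_Fart.
; Tick drives movement, health bar updates and delayed passive regen, while trigger overlaps flip the sprite and direction.
; BP_Projectile overlaps apply damage, computed as Damage minus Health.
; A non-positive result plays a flower explosion and transforms it into a harmless, still-walking form without health bar, attacks or regen.
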(event `PassiveHP`
  (params (Tick :type "Float (double-precision)"))
  (bind _timesinceheal (`self.TimeSinceHeal`))
  ;[1 1 1] Passive HP Regen
  (if (not (`self.Transformed`))
    (bind _output_get (set `self.TimeSinceHit` (+ (`self.TimeSinceHit`) Tick)))
    (if (>= _output_get 5.0)
      (if (>= _timesinceheal 0.2)
        (`self.Increase_Health` 0.2)
        (set `self.TimeSinceHeal` 0.0)
        (else
          (set `self.TimeSinceHeal` (+ _timesinceheal Tick)))))))

(event `SetFlipBookMoving`
  (params (Rotation :type "Float (double-precision)"))
  ;[1 1 1] Pawn Facing Direction
  (if (> Rotation 0.0)
    (`KismetSystemLibrary.PrintString` "greater than 0")
    (`SceneComponent.K2_SetRelativeRotation` (`self.PaperFlipbook`) (struct :`Yaw` 180.0) false false)
    (set `self.Rotation` -1.0)
    (else
      (`KismetSystemLibrary.PrintString` "less than 0")
      (`SceneComponent.K2_SetRelativeRotation` :`self` (`self.PaperFlipbook`))
      (set `self.Rotation` 1.0))))

(event `self.ReceiveActorBeginOverlap`
  (params (OtherActor :type "Actor Object Reference")))

(event `Fart`
  ;[1 1 1] Fart Event
  (if (and (not (`self.Farting`)) (not (`self.Transformed`)))
    (set `self.Farting` true)
    (`|SpawnActorFromClass` "/Game/Blueprints/Enemies/Mushroom/BP_Fart.BP_Fart_C" (`KismetMathLibrary.Conv_VectorToTransform` (`SceneComponent.K2_GetComponentLocation` (`self.CapsuleComponent`))) "Undefined" "OverrideRootScale")
    (`KismetSystemLibrary.Delay` 10.0)
    (set `self.Farting` false)))

(event `self.ReceiveTick`
  (params (DeltaSeconds :type "Float (single-precision)"))
  (`self.Fart`)
  ;[1 1 1] Mushroom health bar
  (if (`self.Transformed`)
    (`ActorComponent.K2_DestroyComponent` (`self.Widget`))
    (else
      (bind _asai_health (cast `/Game/Blueprints/Enemies/AI_Health` (`WidgetComponent.GetUserWidgetObject` (`self.Widget`))))
      (`ProgressBar.SetPercent` (`/Game/Blueprints/Enemies/AI_Health.ProgressBar_54` _asai_health) (`self.Health`))))
  ;[1 1 1] Mushroom Movement
  (`|ExecutionSequence`
    (:`then_0`
      (`self.AddMovementInput` (1.0 0.0 0.0) (* (`self.Rotation`) (`self.My Speed`)) true))
    (:`then_1`
      (`self.PassiveHP` DeltaSeconds))))

(event `self.CapsuleComponent.OnComponentHit`
  (params (OtherActor :type "Actor Object Reference") (OtherComp :type "PrimitiveComponent Object Reference") (NormalImpulse :type "Vector Structure") (Hit :type "HitResult Structure (by ref)"))
  ;[1 1 1] Hit Player
  (if (not (`self.Transformed`))
    (`GameplayStatics.PlaySound2D` null)
    (bind _as2dside_scroller_character (cast `/Game/Blueprints/2DSideScrollerCharacter` OtherActor))
    (if (!= (`PaperFlipbookComponent.GetFlipbook` (`self.PaperFlipbook`)) (`self.GM_Walk2`))
      (`/Game/Blueprints/2DSideScrollerCharacter.Decrease_Health` _as2dside_scroller_character 0.25))))

(event `self.CapsuleComponent.OnComponentBeginOverlap`
  (params (OtherActor :type "Actor Object Reference") (OtherComp :type "PrimitiveComponent Object Reference") (OtherBodyIndex :type Integer) (bFromSweep :type Boolean) (SweepResult :type "HitResult Structure (by ref)"))
  ;[1 1 1] Overlap with trigger boundaries
  (cast `/Game/Blueprints/Enemies/Mushroom/BP_TriggerPoint` OtherActor)
  (`self.SetFlipBookMoving` (`self.Rotation`)))

(event `self.ReceiveAnyDamage`
  (params (Damage :type "Float (single-precision)") (DamageType :type "DamageType Object Reference") (InstigatedBy :type "Controller Object Reference") (DamageCauser :type "Actor Object Reference"))
  (bind _returnvalue (- Damage (`self.Health`)))
  ;[1 1 1] Process Mushroom Damage
  (if (not (`self.Transformed`))
    (set `self.TimeSinceHit` 0.0)
    (if (!= (`PaperFlipbookComponent.GetFlipbook` (`self.PaperFlipbook`)) (`self.GM_Walk2`))
      (`KismetSystemLibrary.PrintString` "mushroom recieved damage")
      (if (<= _returnvalue 0.0)
        (`KismetSystemLibrary.PrintString` "died")
        (set `self.Health` 0.0)
        (`PaperFlipbookComponent.SetFlipbook` (`self.PaperFlipbook`) "/Game/Sprites/Flipbooks/FB_FlowerExplosion.FB_FlowerExplosion")
        (`GameplayStatics.PlaySound2D` "/Game/Sounds/Smoochy+Kiss.Smoochy+Kiss")
        (`SceneComponent.SetRelativeScale3D` (`self.PaperFlipbook`) (1.0 1.0 1.0))
        (`KismetSystemLibrary.Delay` (`PaperFlipbookComponent.GetFlipbookLength` (`self.PaperFlipbook`)))
        (`SceneComponent.SetRelativeScale3D` (`self.PaperFlipbook`) (0.6 0.6 0.6))
        (`PaperFlipbookComponent.SetFlipbook` (`self.PaperFlipbook`) "/Game/Sprites/Flipbooks/GM_walk2.GM_walk2")
        (`PrimitiveComponent.SetCollisionEnabled` (`self.CapsuleComponent`) "QueryOnly")
        (set `self.Transformed` true)
        (else
          (set `self.Health` _returnvalue))))))

(event `self.DamageCapsule.OnComponentBeginOverlap`
  (params (OtherActor :type "Actor Object Reference") (OtherComp :type "PrimitiveComponent Object Reference") (OtherBodyIndex :type Integer) (bFromSweep :type Boolean) (SweepResult :type "HitResult Structure (by ref)"))
  ;[1 1 1] Projectile Damage
  (bind _asbp_projectile (cast `/Game/Blueprints/Deprecated/BP_Projectile` OtherActor))
  (`PrimitiveComponent.SetCollisionEnabled` (`/Game/Blueprints/Deprecated/BP_Projectile.Sphere` _asbp_projectile) "NoCollision")
  (`GameplayStatics.ApplyDamage` self 0.5 null _asbp_projectile))

(event `Increase_Health`
  (params (`Heal Amount` :type "Float (double-precision)"))
  (bind _returnvalue (+ (`self.Health`) `Heal Amount`))
  (if (>= _returnvalue 1.0)
    (set `self.Health` 1.0)
    (else
      (set `self.Health` _returnvalue))))

(fn `UserConstructionScript`)