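; Deprecated Paper2D owl enemy for a side-scroller that, when defeated, plays a flower explosion and transforms into a non-colliding idle form.
; Tick updates its health bar, fires lasers aimed at the player inside LaserBox, paced by flipbook length, and regenerates health after a hit-free delay.
; Projectile overlaps become damage, while capsule hits hurt the player.
; The player knockback logic is disconnected.
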(event `PassiveHP`
  (params (Tick :type "Float (double-precision)"))
  (bind _timesinceheal (`self.TimeSinceHeal`))
  ;[1 1 1] Passive HP Regen
  (if (not (`self.Transformed`))
    (bind _output_get (set `self.TimeSinceHit` (+ (`self.TimeSinceHit`) Tick)))
    (if (>= _output_get 5.0)
      (if (>= _timesinceheal 0.2)
        (`self.Increase_Health` 0.2)
        (set `self.TimeSinceHeal` 0.0)
        (else
          (set `self.TimeSinceHeal` (+ _timesinceheal Tick)))))))

(event `self.ReceiveTick`
  (params (DeltaSeconds :type "Float (single-precision)"))
  (bind _returnvalue (`SceneComponent.K2_GetComponentLocation` (`self.Eye`)))
  ;[1 1 1] Owl health bar
  (if (`self.Transformed`)
    (`ActorComponent.K2_DestroyComponent` (`self.Widget`))
    (else
      (bind _asai_health (cast `/Game/Blueprints/Enemies/AI_Health` (`WidgetComponent.GetUserWidgetObject` (`self.Widget`))))
      (`ProgressBar.SetPercent` (`/Game/Blueprints/Enemies/AI_Health.ProgressBar_54` _asai_health) (`self.Health`))))
  (`|ExecutionSequence`
    (:`then_0`
      (if (and (`self.Inside`) (not (`self.Shooting`)) (> (`self.Health`) 0.0))
        (set `self.Shooting` true)
        (bind _as2dside_scroller_character (cast `/Game/Blueprints/2DSideScrollerCharacter` (`GameplayStatics.GetPlayerPawn` 0)))
        (`PaperFlipbookComponent.SetFlipbook` (`self.PaperFlipbook`) "/Game/Sprites/Flipbooks/FB_Owl_Evil_Shoot.FB_Owl_Evil_Shoot")
        (`KismetSystemLibrary.PrintString` "Hello")
        (`|SpawnActorFromClass` "/Game/Blueprints/Enemies/BP_Laser.BP_Laser_C" (`KismetMathLibrary.MakeTransform` _returnvalue (`KismetMathLibrary.FindLookAtRotation` _returnvalue (`self.K2_GetActorLocation` _as2dside_scroller_character))) "Undefined" "OverrideRootScale")
        (`KismetSystemLibrary.Delay` (`PaperFlipbookComponent.GetFlipbookLength` (`self.PaperFlipbook`)))
        (set `self.Shooting` false)
        (if (> (`self.Health`) 0.0)
          (`PaperFlipbookComponent.SetFlipbook` (`self.PaperFlipbook`) "/Game/Sprites/Flipbooks/FB_Owl_Evil_Idle.FB_Owl_Evil_Idle")
          (else
            (`PaperFlipbookComponent.SetFlipbook` (`self.PaperFlipbook`) "/Game/Sprites/Flipbooks/GO_Idle2.GO_Idle2")))))
    (:`then_1`
      (`self.PassiveHP` DeltaSeconds))))

(event `self.ReceiveBeginPlay`
  ;[1 1 1] Owl health bar
)

(event `self.ReceiveActorBeginOverlap`
  (params (OtherActor :type "Actor Object Reference")))

(event `self.CapsuleComponent.OnComponentHit`
  (params (OtherActor :type "Actor Object Reference") (OtherComp :type "PrimitiveComponent Object Reference") (NormalImpulse :type "Vector Structure") (Hit :type "HitResult Structure (by ref)"))
  ;[1 1 1] Hurt Player
  (if (> (`self.Health`) 0.0)
    (`GameplayStatics.PlaySound2D` null)
    (bind _as2dside_scroller_character (cast `/Game/Blueprints/2DSideScrollerCharacter` OtherActor))
    (`/Game/Blueprints/2DSideScrollerCharacter.Decrease_Health` _as2dside_scroller_character 0.25)))

(event `self.ReceiveAnyDamage`
  (params (Damage :type "Float (single-precision)") (DamageType :type "DamageType Object Reference") (InstigatedBy :type "Controller Object Reference") (DamageCauser :type "Actor Object Reference"))
  (bind _returnvalue (- (`self.Health`) Damage))
  ;[1 1 1] Process Owl Damage
  (if (not (`self.Transformed`))
    (set `self.TimeSinceHit` 0.0)
    (`KismetSystemLibrary.PrintString` "received damage")
    (if (<= _returnvalue 0.0)
      (if (not (`self.Transformed`))
        (`KismetSystemLibrary.PrintString` "died")
        (set `self.Transformed` true)
        (set `self.Health` 0.0)
        (`PaperFlipbookComponent.SetFlipbook` (`self.PaperFlipbook`) "/Game/Sprites/Flipbooks/FB_FlowerExplosion.FB_FlowerExplosion")
        (`GameplayStatics.PlaySound2D` "/Game/Sounds/Smoochy+Kiss.Smoochy+Kiss")
        (`SceneComponent.SetRelativeScale3D` (`self.PaperFlipbook`) (1.0 1.0 1.0))
        (`KismetSystemLibrary.Delay` (`PaperFlipbookComponent.GetFlipbookLength` (`self.PaperFlipbook`)))
        (`SceneComponent.SetRelativeScale3D` (`self.PaperFlipbook`) (0.45 0.45 0.45))
        (`PaperFlipbookComponent.SetFlipbook` (`self.PaperFlipbook`) "/Game/Sprites/Flipbooks/GO_Idle2.GO_Idle2")
        (`PrimitiveComponent.SetCollisionEnabled` (`self.CapsuleComponent`) "NoCollision"))
      (else
        (set `self.Health` _returnvalue)
        (`PaperFlipbookComponent.SetFlipbook` (`self.PaperFlipbook`) "/Game/Sprites/Flipbooks/FB_Owl_Evil_Hit.FB_Owl_Evil_Hit")
        (`KismetSystemLibrary.Delay` (`PaperFlipbookComponent.GetFlipbookLength` (`self.PaperFlipbook`)))
        (if (`self.Transformed`)
          (`PaperFlipbookComponent.SetFlipbook` (`self.PaperFlipbook`) "/Game/Sprites/Flipbooks/GO_Idle2.GO_Idle2")
          (else
            (`PaperFlipbookComponent.SetFlipbook` (`self.PaperFlipbook`) "/Game/Sprites/Flipbooks/FB_Owl_Evil_Idle.FB_Owl_Evil_Idle")))))))

(event `self.Laser Box.OnComponentBeginOverlap`
  (params (OtherActor :type "Actor Object Reference") (OtherComp :type "PrimitiveComponent Object Reference") (OtherBodyIndex :type Integer) (bFromSweep :type Boolean) (SweepResult :type "HitResult Structure (by ref)"))
  (cast `/Game/Blueprints/2DSideScrollerCharacter` OtherActor)
  (set `self.Inside` true))

(event `self.Laser Box.OnComponentEndOverlap`
  (params (OtherActor :type "Actor Object Reference") (OtherComp :type "PrimitiveComponent Object Reference") (OtherBodyIndex :type Integer))
  (cast `/Game/Blueprints/2DSideScrollerCharacter` OtherActor)
  (set `self.Inside` false))

(event `self.DamageCollision.OnComponentBeginOverlap`
  (params (OtherActor :type "Actor Object Reference") (OtherComp :type "PrimitiveComponent Object Reference") (OtherBodyIndex :type Integer) (bFromSweep :type Boolean) (SweepResult :type "HitResult Structure (by ref)"))
  (bind _asbp_projectile (cast `/Game/Blueprints/Deprecated/BP_Projectile` OtherActor))
  (`PrimitiveComponent.SetCollisionEnabled` (`/Game/Blueprints/Deprecated/BP_Projectile.Sphere` _asbp_projectile) "NoCollision")
  (`GameplayStatics.ApplyDamage` self 0.5 null _asbp_projectile))

(event `Increase_Health`
  (params (`Heal Amount` :type "Float (double-precision)"))
  (bind _returnvalue (+ (`self.Health`) `Heal Amount`))
  (if (>= _returnvalue 1.0)
    (set `self.Health` 1.0)
    (else
      (set `self.Health` _returnvalue))))

(fn `UserConstructionScript`)