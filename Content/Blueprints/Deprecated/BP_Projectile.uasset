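; Projectile, filed under Deprecated, that bursts when its sphere overlaps any actor other than the 2D side-scroller character.
; On overlap it activates its particle system, stops movement and attaches to the actor it touched.
; A timeline then resizes the sphere's radius with overlap updates, as an area burst, and destroys the projectile when finished.
; It deals no damage itself: the Hit event is empty, and the enemy-damage, ApplyDamage and older Grow timeline chains are unwired.
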(event `self.ReceiveBeginPlay`)

(event `self.ReceiveActorBeginOverlap`
  (params (OtherActor :type "Actor Object Reference")))

(event `self.ReceiveTick`
  (params (DeltaSeconds :type "Float (single-precision)")))

(event `self.ReceiveHit`
  (params (MyComp :type "PrimitiveComponent Object Reference") (Other :type "Actor Object Reference") (OtherComp :type "PrimitiveComponent Object Reference") (bSelfMoved :type Boolean) (HitLocation :type "Vector Structure") (HitNormal :type "Vector Structure") (NormalImpulse :type "Vector Structure") (Hit :type "HitResult Structure (by ref)")))

(event `self.Sphere.OnComponentBeginOverlap`
  (params (OtherActor :type "Actor Object Reference") (OtherComp :type "PrimitiveComponent Object Reference") (OtherBodyIndex :type Integer) (bFromSweep :type Boolean) (SweepResult :type "HitResult Structure (by ref)"))
  (if (!= OtherActor "/Game/Blueprints/2DSideScrollerCharacter.2DSideScrollerCharacter")
    (`ActorComponent.Activate` (`self.ParticleSystem`) false)
    (`MovementComponent.StopMovementImmediately` (`self.ProjectileMovement`))
    (`self.K2_AttachRootComponentToActor` OtherActor)
    (bind (_direction _size) (`Timeline|Timeline_0` :!via `PlayFromStart`)
      (:`Update`
        (`SphereComponent.SetSphereRadius` (`self.Sphere`) _size true))
      (:`Finished`
        (`self.K2_DestroyActor`)))))

(fn `UserConstructionScript`)