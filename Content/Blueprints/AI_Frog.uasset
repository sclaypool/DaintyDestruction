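; Evil frog enemy for the 2D side-scroller that hops back and forth and hurts the player on capsule hit.
; Tick launches each hop, and landing flips direction after an idle delay.
; Projectiles overlapping its damage capsule hurt it, while Tick regenerates health after an initial timer that hits never reset.
; At zero health it stops hopping, plays a flower-explosion kiss transformation and loses capsule collision; player knockback logic is unwired.
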(event `self.ReceiveBeginPlay`)

(event `self.ReceiveActorBeginOverlap`
  (params (OtherActor :type "Actor Object Reference")))

(event `self.OnLanded`
  (params (Hit :type "HitResult Structure (by ref)"))
  (set `self.Jumping` false)
  (`PaperFlipbookComponent.SetFlipbook` (`self.PaperFlipbook`) "/Game/Sprites/Flipbooks/FB_Frog_Evil_Idle.FB_Frog_Evil_Idle")
  (if (> (`self.Rotation`) 0.0)
    (`SceneComponent.K2_SetRelativeRotation` :`self` (`self.PaperFlipbook`))
    (else
      (`SceneComponent.K2_SetRelativeRotation` (`self.PaperFlipbook`) (struct :`Yaw` 180.0) false false)))
  (`KismetSystemLibrary.Delay` (* (`PaperFlipbookComponent.GetFlipbookLength` (`self.PaperFlipbook`)) 2.0))
  (set `self.Rotation` (* (`self.Rotation`) -1.0))
  (set `self.Idle` true))

(event `self.ReceiveTick`
  (params (DeltaSeconds :type "Float (single-precision)"))
  (bind _timesinceheal (`self.TimeSinceHeal`))
  (`|ExecutionSequence`
    (:`then_0`
      (if (and (`self.Idle`) (not (`self.Jumping`)) (not (`self.Transformed`)))
        (set `self.Idle` false)
        (set `self.Jumping` true)
        (`PaperFlipbookComponent.SetFlipbook` (`self.PaperFlipbook`) "/Game/Sprites/Flipbooks/FB_Frog_Evil_Jump.FB_Frog_Evil_Jump")
        (`self.LaunchCharacter` (`KismetMathLibrary.MakeVector` (* (`self.Rotation`) -200.0) 0.0 200.0))))
    (:`then_1`
      ;[1 1 1] Passive HP Regen
      (bind _output_get (set `self.TimeSinceHit` (+ (`self.TimeSinceHit`) DeltaSeconds)))
      (if (>= _output_get 5.0)
        (if (>= _timesinceheal 0.2)
          (`self.Increase_Health` 0.2)
          (set `self.TimeSinceHeal` 0.0)
          (else
            (set `self.TimeSinceHeal` (+ _timesinceheal DeltaSeconds))))))))

(event `Increase_Health`
  (params (`Heal Amount` :type "Float (double-precision)"))
  (bind _returnvalue (+ (`self.Health`) `Heal Amount`))
  (if (>= _returnvalue 1.0)
    (set `self.Health` 1.0)
    (else
      (set `self.Health` _returnvalue))))

(event `self.CapsuleComponent.OnComponentHit`
  (params (OtherActor :type "Actor Object Reference") (OtherComp :type "PrimitiveComponent Object Reference") (NormalImpulse :type "Vector Structure") (Hit :type "HitResult Structure (by ref)"))
  ;[1 1 1] Hurt Player
  (if (> (`self.Health`) 0.0)
    (bind _as2dside_scroller_character (cast `/Game/Blueprints/2DSideScrollerCharacter` OtherActor))
    (`/Game/Blueprints/2DSideScrollerCharacter.Decrease_Health` _as2dside_scroller_character 0.25)))

(event `self.ReceiveAnyDamage`
  (params (Damage :type "Float (single-precision)") (DamageType :type "DamageType Object Reference") (InstigatedBy :type "Controller Object Reference") (DamageCauser :type "Actor Object Reference"))
  (bind _returnvalue (- (`self.Health`) Damage))
  ;[1 1 1] Process Frog Damage
  (`KismetSystemLibrary.PrintString` "received damage")
  (if (<= _returnvalue 0.0)
    (set `self.Transformed` true)
    (`KismetSystemLibrary.PrintString` "died")
    (set `self.Health` 0.0)
    (`PaperFlipbookComponent.SetFlipbook` (`self.PaperFlipbook`) "/Game/Sprites/Flipbooks/FB_FlowerExplosion.FB_FlowerExplosion")
    (`GameplayStatics.PlaySound2D` "/Game/Sounds/Smoochy+Kiss.Smoochy+Kiss")
    (`SceneComponent.SetRelativeScale3D` (`self.PaperFlipbook`) (1.0 1.0 1.0))
    (`KismetSystemLibrary.Delay` (`PaperFlipbookComponent.GetFlipbookLength` (`self.PaperFlipbook`)))
    (`SceneComponent.SetRelativeScale3D` (`self.PaperFlipbook`) (0.45 0.45 0.45))
    (`PaperFlipbookComponent.SetFlipbook` (`self.PaperFlipbook`) "/Game/Sprites/Flipbooks/GF_Idle2.GF_Idle2")
    (`PrimitiveComponent.SetCollisionEnabled` (`self.CapsuleComponent`) "NoCollision")
    (else
      (set `self.Health` _returnvalue)
      (`PaperFlipbookComponent.SetFlipbook` (`self.PaperFlipbook`) "/Game/Sprites/Flipbooks/FB_Frog_Evil_Hit.FB_Frog_Evil_Hit")
      (`KismetSystemLibrary.Delay` (`PaperFlipbookComponent.GetFlipbookLength` (`self.PaperFlipbook`)))
      (`PaperFlipbookComponent.SetFlipbook` (`self.PaperFlipbook`) "/Game/Sprites/Flipbooks/FB_Frog_Evil_Idle.FB_Frog_Evil_Idle")
      (if (<= (`self.Health`) 0.0)
        (`PaperFlipbookComponent.SetFlipbook` (`self.PaperFlipbook`) "/Game/Sprites/Flipbooks/GF_Idle2.GF_Idle2")))))

(event `self.DamageCapsule.OnComponentBeginOverlap`
  (params (OtherActor :type "Actor Object Reference") (OtherComp :type "PrimitiveComponent Object Reference") (OtherBodyIndex :type Integer) (bFromSweep :type Boolean) (SweepResult :type "HitResult Structure (by ref)"))
  (bind _asbp_projectile (cast `/Game/Blueprints/BP_Projectile` OtherActor))
  (`PrimitiveComponent.SetCollisionEnabled` (`/Game/Blueprints/BP_Projectile.Sphere` _asbp_projectile) "NoCollision")
  (`GameplayStatics.ApplyDamage` self 0.3 null _asbp_projectile))

(fn `UserConstructionScript`)