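; BP_Layout is a tile spawner that lays out a straight row of randomized environment tiles when play begins.
; BeginPlay loops over NumberToSpawn, using Type to select the Forest or Cave set and randomly picking one of its two tile classes at each step.
; Tiles start at the actor's location and step along world X at a fixed spacing, ignoring the actor's rotation and scale.
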(event `self.ReceiveBeginPlay`
  (bind _returnvalue (`KismetMathLibrary.RandomIntegerInRange` 0 1))
  (for _index (range (+ (`self.NumberToSpawn`) 1))
    (switch `/Game/Blueprints/Environment/Tiles/TileType` (`self.Type`)
      (:`NewEnumerator0`
        (switch `int` _returnvalue
          (:`0`
            (bind _returnvalue_2 (`KismetMathLibrary.MakeTransform` (+ (`self.K2_GetActorLocation`) (`KismetMathLibrary.MakeVector` (* _index 230.0)))))
            (`|SpawnActorFromClass` "/Game/Blueprints/Environment/Tiles/Tile_Forest_1.Tile_Forest_1_C" _returnvalue_2 "Undefined" "OverrideRootScale"))
          (:`1`
            (`|SpawnActorFromClass` "/Game/Blueprints/Environment/Tiles/Tile_Forest_2.Tile_Forest_2_C" _returnvalue_2 "Undefined" "OverrideRootScale"))))
      (:`NewEnumerator1`
        (switch `int` _returnvalue
          (:`0`
            (`|SpawnActorFromClass` "/Game/Blueprints/Environment/Tiles/Tile_Cave_1.Tile_Cave_1_C" _returnvalue_2 "Undefined" "OverrideRootScale"))
          (:`1`
            (`|SpawnActorFromClass` "/Game/Blueprints/Environment/Tiles/Tile_Cave_2.Tile_Cave_2_C" _returnvalue_2 "Undefined" "OverrideRootScale")))))))

(event `self.ReceiveActorBeginOverlap`
  (params (OtherActor :type "Actor Object Reference")))

(event `self.ReceiveTick`
  (params (DeltaSeconds :type "Float (single-precision)")))

(fn `UserConstructionScript`)