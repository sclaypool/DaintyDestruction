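; Base moving platform for a side-scroller that shuttles between two placed location actors and transforms when the character or a glitter touches it.
; Tick calls Move, which alternates MoveComponentTo targets on the root over Speed, with a flag and fixed short delay gating each flip.
; Overlapping the Transform component swaps the flipbook to its good version, offsets it and calls UpdateCharacter unless already Transformed; glitter also triggers its own growth.
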(event `self.ReceiveBeginPlay`)

(event `Move`
  (bind _defaultsceneroot (`self.DefaultSceneRoot`))
  (if (not (`self.Moving`))
    (set `self.Moving` true)
    (switch `int` (`self.LocationNum`)
      (:`0`
        (`KismetSystemLibrary.MoveComponentTo` _defaultsceneroot (`self.K2_GetActorLocation` (`self.Location1`)) (struct) false false (`self.Speed`))
        (`KismetSystemLibrary.Delay` 0.4)
        (set `self.Moving` false)
        (set `self.LocationNum` 1))
      (:`1`
        (`KismetSystemLibrary.MoveComponentTo` _defaultsceneroot (`self.K2_GetActorLocation` (`self.Location2`)) (struct) false false (`self.Speed`))
        (`KismetSystemLibrary.Delay` 0.4)
        (set `self.Moving` false)
        (set `self.LocationNum` 0)))))

(event `self.ReceiveActorBeginOverlap`
  (params (OtherActor :type "Actor Object Reference")))

(event `self.ReceiveTick`
  (params (DeltaSeconds :type "Float (single-precision)"))
  (`self.Move`))

(event `self.Transform.OnComponentBeginOverlap`
  (params (OtherActor :type "Actor Object Reference") (OtherComp :type "PrimitiveComponent Object Reference") (OtherBodyIndex :type Integer) (bFromSweep :type Boolean) (SweepResult :type "HitResult Structure (by ref)"))
  (cast `/Game/Blueprints/2DSideScrollerCharacter` OtherActor
    (:`then`
      (if (not (`self.Transformed`)) :!label _label
        (`PaperFlipbookComponent.SetFlipbook` (`self.PaperFlipbook`) "/Game/Sprites/Flipbooks/FB_Platform_Moving_Good.FB_Platform_Moving_Good")
        (`SceneComponent.K2_AddLocalOffset` (`self.PaperFlipbook`) (0.0 -40.0 0.0) false false)
        (`self.UpdateCharacter`)))
    (:`CastFailed`
      (bind _asbp_glitter (cast `/Game/Blueprints/Enemies/BP_Glitter` OtherActor))
      (`|ExecutionSequence`
        (:`then_0`
          (`/Game/Blueprints/Enemies/BP_Glitter.TriggerGrowth` _asbp_glitter))
        (:`then_1`
          (goto _label))))))

(fn `UserConstructionScript`
  (`parent.UserConstructionScript`))