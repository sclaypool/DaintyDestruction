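; Base Blueprint for a still platform that turns from bad to good when the side-scroller character or a glitter actor touches it.
; The construction script applies the bad sprite, and an overlap on TransformSection swaps in the good one.
; A Transformed flag limits the swap and its following UpdateCharacter call to one time.
; Glitter overlaps also trigger that glitter's growth, even if the platform has already transformed.
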(event `self.ReceiveBeginPlay`)

(event `self.ReceiveActorBeginOverlap`
  (params (OtherActor :type "Actor Object Reference")))

(event `self.ReceiveTick`
  (params (DeltaSeconds :type "Float (single-precision)")))

(event `self.TransformSection.OnComponentBeginOverlap`
  (params (OtherActor :type "Actor Object Reference") (OtherComp :type "PrimitiveComponent Object Reference") (OtherBodyIndex :type Integer) (bFromSweep :type Boolean) (SweepResult :type "HitResult Structure (by ref)"))
  (cast `/Game/Blueprints/2DSideScrollerCharacter` OtherActor
    (:`then`
      (if (not (`self.Transformed`)) :!label _label
        (`PaperSpriteComponent.SetSprite` (`self.Platform`) (`self.GoodPlatform`))
        (set `self.Transformed` true)
        (`self.UpdateCharacter`)))
    (:`CastFailed`
      (bind _asbp_glitter (cast `/Game/Blueprints/Enemies/BP_Glitter` OtherActor))
      (`|ExecutionSequence`
        (:`then_0`
          (`/Game/Blueprints/Enemies/BP_Glitter.TriggerGrowth` _asbp_glitter))
        (:`then_1`
          (goto _label))))))

(fn `UserConstructionScript`
  (`PaperSpriteComponent.SetSprite` (`self.Platform`) (`self.BadPlatform`)))