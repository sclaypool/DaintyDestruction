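; Easter egg pickup for the 2D side scroller that swaps sprite and plays a sparkle when the player enters its sphere.
; The character's PickupItem event adds its ItemInfo, built in the construction script, to the HUD inventory if in range, then disables collision.
; EquipAction spawns BP_HatTest at the character's equip location, hiding it after a delay, with a counter blocking overlapping spawns.
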(event `self.ReceiveBeginPlay`
  ;[1 1 1] Pickup and add item to inventory
  (bind _as2dside_scroller_character (cast `/Game/Blueprints/2DSideScrollerCharacter` (`GameplayStatics.GetPlayerCharacter` 0)))
  (set `self.MyCharacter` _as2dside_scroller_character)
  (add `/Game/Blueprints/2DSideScrollerCharacter.PickupItem` _as2dside_scroller_character (delegate `PickupItem_Event_0`)))

(event `PickupItem_Event_0`
  (bind _hudreference (`/Game/Blueprints/2DSideScrollerCharacter.HUDReference` (`self.MyCharacter`)))
  ;[1 1 1] Pickup and add item to inventory
  (if (and (`self.GetActorEnableCollision`) (`self.IsInRange`))
    (`KismetArrayLibrary.Array_Add` (`/Game/Blueprints/HUD.Inventory` _hudreference) (`self.ItemInfo`))
    (`self.SetActorHiddenInGame` self false)
    (`self.SetActorEnableCollision` false)
    (`/Game/Blueprints/HUD.RefreshInventory` _hudreference)))

(event `self.Sphere.OnComponentBeginOverlap`
  (params (OtherActor :type "Actor Object Reference") (OtherComp :type "PrimitiveComponent Object Reference") (OtherBodyIndex :type Integer) (bFromSweep :type Boolean) (SweepResult :type "HitResult Structure (by ref)"))
  ;[1 1 1] Triggers
  (cast `/Game/Blueprints/2DSideScrollerCharacter` OtherActor)
  (set `self.IsInRange` true)
  (`PaperSpriteComponent.SetSprite` (`self.EasterEgg`) "/Game/Sprites/EasterEggs/EasterEgg04_Sprite_0.EasterEgg04_Sprite_0")
  (`GameplayStatics.PlaySoundAtLocation` "/Game/Sounds/Sparkle.Sparkle"))

(event `self.Sphere.OnComponentEndOverlap`
  (params (OtherActor :type "Actor Object Reference") (OtherComp :type "PrimitiveComponent Object Reference") (OtherBodyIndex :type Integer))
  ;[1 1 1] Triggers
  (cast `/Game/Blueprints/2DSideScrollerCharacter` OtherActor)
  (set `self.IsInRange` false))

(event `/Game/Blueprints/Inventory/ActionInterface.EquipAction`
  (if (< (`self.numberOfSpawns`) 1)
    (bind _output_get (set `self.numberOfSpawns` (+ (`self.numberOfSpawns`) 1)))
    (`KismetSystemLibrary.PrintString` (`KismetStringLibrary.Conv_IntToString` _output_get))
    (bind _returnvalue (`|SpawnActorFromClass` "/Game/Blueprints/Inventory/BP_HatTest.BP_HatTest_C" (`SceneComponent.K2_GetComponentToWorld` (`/Game/Blueprints/2DSideScrollerCharacter.EquipLocation` (`self.MyCharacter`))) "Undefined" "OverrideRootScale"))
    (`KismetSystemLibrary.Delay` 5.0)
    (bind _output_get_2 (set `self.numberOfSpawns` (- (`self.numberOfSpawns`) 1)))
    (`KismetSystemLibrary.PrintString` (`KismetStringLibrary.Conv_IntToString` _output_get_2))
    (`self.SetActorHiddenInGame` _returnvalue true)))

(event `self.ReceiveActorBeginOverlap`
  (params (OtherActor :type "Actor Object Reference")))

(event `self.ReceiveTick`
  (params (DeltaSeconds :type "Float (single-precision)")))

(fn `UserConstructionScript`
  (setmembers `/Game/Blueprints/Inventory/InventoryStruct` :`StructRef` (`self.ItemInfo`) :`Item` self :`ItemImage` (`self.Inventory Image`) :`ActionText` (`self.ActionText`))
  (`PaperSpriteComponent.SetSprite` (`self.EasterEgg`) (`self.CustomMesh`)))