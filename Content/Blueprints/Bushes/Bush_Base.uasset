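; Bush_Base is a base Paper2D bush that starts dead and grows when the side-scroller player character touches it.
; The construction script sets the flipbook to the Dead animation.
; On the first Box overlap by 2DSideScrollerCharacter, a Transformed flag locks the change in, the Transform flipbook plays, and after a delay of that flipbook's length the bush switches to Grown.
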(event `self.ReceiveBeginPlay`)

(event `self.ReceiveActorBeginOverlap`
  (params (OtherActor :type "Actor Object Reference")))

(event `self.ReceiveTick`
  (params (DeltaSeconds :type "Float (single-precision)")))

(event `self.Box.OnComponentBeginOverlap`
  (params (OtherActor :type "Actor Object Reference") (OtherComp :type "PrimitiveComponent Object Reference") (OtherBodyIndex :type Integer) (bFromSweep :type Boolean) (SweepResult :type "HitResult Structure (by ref)"))
  (if (not (`self.Transformed`))
    (cast `/Game/Blueprints/2DSideScrollerCharacter` OtherActor)
    (set `self.Transformed` true)
    (`PaperFlipbookComponent.SetFlipbook` (`self.PaperFlipbook`) (`self.Transform`))
    (`KismetSystemLibrary.Delay` (`PaperFlipbookComponent.GetFlipbookLength` (`self.PaperFlipbook`)))
    (`PaperFlipbookComponent.SetFlipbook` (`self.PaperFlipbook`) (`self.Grown`))))

(fn `UserConstructionScript`
  (`PaperFlipbookComponent.SetFlipbook` (`self.PaperFlipbook`) (`self.Dead`)))